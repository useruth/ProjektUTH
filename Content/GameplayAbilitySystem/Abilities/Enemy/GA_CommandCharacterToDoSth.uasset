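; Gameplay ability and planner action in which the boss NPC orders another NPC to power an empty energy storage.
; It picks the first other NPC, waves, adds an obey goal and awaits check-in, then yells; the "Order" notify swaps that goal for provide-energy.
; It ends once the storage has energy.
; Planner overrides advertise an energy-level effect, requiring the agent's held object to be null.
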(event `self.K2_ActivateAbility`
  (bind _returnvalue (`self.GetAvatarActorFromActorInfo`))
  (bind _returnvalue_2 (`self.GetAvatarActorFromActorInfo`))
  (`self.SetCanBeCanceled` true)
  (`self.K2_CommitAbility`)
  (if (not (> (`/Game/Blueprints/BP_EnergyStorage.CurrentEnergy` (`self.TargetInteractionObject`)) 0.0))
    (bind _character (`self.GetSuitableCharacter` (cast `/Game/Blueprints/BP_BHCharacterBase` (`self.GetAvatarActorFromActorInfo`) :!pure true)))
    (set `self.CachedCharacter` _character)
    (set `/Game/Blueprints/BP_BHNPC_Boss.RequiredCharacter` (`self.CachedCharacter`) (cast `/Game/Blueprints/BP_BHNPC_Boss` (`self.GetAvatarActorFromActorInfo`) :!pure true))
    (`Actor.K2_SetActorRotation` (cast `/Game/Blueprints/BP_BHCharacterBase` _returnvalue_2 :!pure true) (`KismetMathLibrary.MakeRotator` 0.0 0.0 (.yaw (`KismetMathLibrary.FindLookAtRotation` (`Actor.K2_GetActorLocation` _returnvalue_2) (`Actor.K2_GetActorLocation` (`self.CachedCharacter`))))) false)
    (`AbilityTask_PlayMontageAndWait.CreatePlayMontageAndWaitProxy` "None" "/Game/Animations/Waving_Montage.Waving_Montage"
      (:`OnCompleted`
        _)
      (:`OnInterrupted`
        _)
      (:`OnCancelled`
        _))
    (`BHPlanner.AddGoal` (`/Game/Blueprints/BP_BHNPCCharacterBase.BHPlanner` (`self.CachedCharacter`)) "/Game/Blueprints/AI/Goals/BP_Goal_ObeyBoss.BP_Goal_ObeyBoss_C")
    (`AbilityTask_WaitGameplayEvent.WaitGameplayEvent` (struct :`TagName` "Event.CheckIn") null
      (:`EventReceived`
        (`Actor.K2_SetActorRotation` (cast `/Game/Blueprints/BP_BHCharacterBase` _returnvalue :!pure true) (`KismetMathLibrary.MakeRotator` 0.0 0.0 (.yaw (`KismetMathLibrary.FindLookAtRotation` (`Actor.K2_GetActorLocation` _returnvalue) (`Actor.K2_GetActorLocation` (`self.CachedCharacter`))))) false)
        (bind _notifyname (`|PlayMontage` (`Actor.GetComponentByClass` (`self.GetAvatarActorFromActorInfo`) "/Script/Engine.SkeletalMeshComponent") "/Game/Animations/Yelling_Montage.Yelling_Montage")
          (:`OnCompleted`
            (if (> (`/Game/Blueprints/BP_EnergyStorage.CurrentEnergy` (`self.TargetInteractionObject`)) 0.0) :!label _label
              (`self.K2_EndAbility`)
              (else
                (add `/Game/Blueprints/BP_EnergyStorage.EnergyStorageStateChangedED` (`self.TargetInteractionObject`) (`|CreateDelegate` :!event `EnergyStorageStateChanged`)))))
          (:`OnInterrupted`
            (goto _label))
          (:`OnNotifyBegin`
            (if (== _notifyname "Order")
              (`AbilitySystemBlueprintLibrary.SendGameplayEventToActor` (`self.CachedCharacter`) (struct :`TagName` "Event.CheckOut"))
              (`BHPlanner.RemoveGoal` (`/Game/Blueprints/BP_BHNPCCharacterBase.BHPlanner` (`self.CachedCharacter`)) "/Game/Blueprints/AI/Goals/BP_Goal_ObeyBoss.BP_Goal_ObeyBoss_C")
              (`BHPlanner.AddGoal` (`/Game/Blueprints/BP_BHNPCCharacterBase.BHPlanner` (`self.CachedCharacter`)) "/Game/Blueprints/AI/Goals/BP_Goal_ProvideEnergy.BP_Goal_ProvideEnergy_C"))))))
    (else
      (`self.K2_EndAbility`))))

(event `EnergyStorageStateChanged`
  (params (Active :type Boolean))
  (if Active
    (`self.K2_EndAbility`)))

(event `self.K2_OnEndAbility`
  (params (bWasCancelled :type Boolean))
  (bind _asbp_bhcharacter_base (cast `/Game/Blueprints/BP_BHCharacterBase` (`self.GetAvatarActorFromActorInfo`) :!pure true))
  (remove `/Game/Blueprints/BP_EnergyStorage.EnergyStorageStateChangedED` (`self.TargetInteractionObject`) (`|CreateDelegate` :!event `EnergyStorageStateChanged`))
  ;[1 1 1] if was canceled this goal maybe wasnt removed
  (`BHPlanner.RemoveGoal` (`/Game/Blueprints/BP_BHNPCCharacterBase.BHPlanner` (`self.CachedCharacter`)) "/Game/Blueprints/AI/Goals/BP_Goal_ObeyBoss.BP_Goal_ObeyBoss_C")
  ;[0 0.8877 1] @TODO: implement special ability task for playing montage with notify exec; then this function can be removed
  (`Character.StopAnimMontage` _asbp_bhcharacter_base (`Character.GetCurrentMontage` _asbp_bhcharacter_base))
  (`parent.K2_OnEndAbility` bWasCancelled))

(event `self.SetActionTargetData`
  (params (TargetData :type "BHWorldStateData Structure"))
  (set `self.TargetInteractionObject` (cast `/Game/Blueprints/BP_EnergyStorage` (`.WorldStateActor` (break `BHWorldStateKey` (`.WorldStateKey` (break `BHWorldStateData` TargetData)))) :!pure true)))

(fn `CanChangeWorldState`
  (params (DesiredWorldState :type "BHWorldStateData Structure") (AgentActor :type "Actor Object Reference"))
  (returns (ReturnValue :type Boolean))
  (bind (_worldstatekey _worldstatevalue) (break `BHWorldStateData` DesiredWorldState))
  (bind (_worldstateactor _worldstatedatatag) (break `BHWorldStateKey` _worldstatekey))
  (if (and (`.bSuccess` (cast `/Game/Blueprints/BP_EnergyStorage` _worldstateactor :!pure true)) (== _worldstatedatatag (`self.EnergyLevelWorldStateTag`)))
    (bind _returnvalue (`BHWorldStateFunctionLibrary.GetWorldStateValueAsFloat` _worldstatevalue))
    (return (`KismetMathLibrary.NearlyEqual_FloatFloat` _returnvalue 1.0))
    (else
      (return false))))

(fn `GetActionCost`
  (params (DesiredWorldState :type "BHWorldStateData Structure") (AgentActor :type "Actor Object Reference") (WithCurrentWorldState :type "Array of BHWorldStateData Structure (by ref)"))
  (returns (ReturnValue :type Integer))
  (return (`self.ActionCost`)))

(fn `GetActionEffectWithContextActor`
  (params (AgentActor :type "Actor Object Reference") (TargetActor :type "Actor Object Reference"))
  (returns (EffectWorldState :type "BHWorldStateData Structure") (ReturnValue :type Boolean))
  (locals (LAgent :type "Actor Object Reference") (LTarget :type "Actor Object Reference") (LWorldStateProvider :type "BHWorldStateProvider Object Reference"))
  (set `local.LAgent` AgentActor)
  (set `local.LTarget` TargetActor)
  (bind _output_get (set `local.LWorldStateProvider` (`Actor.GetComponentByClass` (`local.LTarget`) "/Script/BrainHacker.BHWorldStateProvider")))
  (`/Engine/EditorBlueprintResources/StandardMacros.IsValid` _output_get
    (:`Is Valid`
      (bind _returnvalue (`BHWorldStateProvider.HasWorldStateValue` (`local.LWorldStateProvider`) (`self.EnergyLevelWorldStateTag`)))
      (if _returnvalue
        (bind _result (`BHWorldStateFunctionLibrary.SetWorldStateValue` (make `BHWorldStateValue`) (`self.WorldStateEnergyLevelEffect`)))
        (return (make `BHWorldStateData` (make `BHWorldStateKey` (`local.LTarget`) (`self.EnergyLevelWorldStateTag`)) _result) true)
        (else
          (return (struct) false))))
    (:`Is Not Valid`
      (return (struct) false))))

(fn `GetSuitableCharacter`
  (params (Instigator :type "/Game/Blueprints/BP_BHCharacterBase Object Reference"))
  (returns (Character :type "/Game/Blueprints/BP_BHNPCCharacterBase Object Reference"))
  (bind _outactors (`GameplayStatics.GetAllActorsOfClass` "/Game/Blueprints/BP_BHNPCCharacterBase.BP_BHNPCCharacterBase_C"))
  (for _array_element _outactors
    (if (!= _array_element Instigator)
      (return _array_element)))
  (return null))

(fn `GetWorldStatePreconditions`
  (params (ForDesiredWorldState :type "BHWorldStateData Structure") (AgentActor :type "Actor Object Reference"))
  (returns (ReturnValue :type "Array of BHWorldStateData Structure"))
  (bind _result (`BHWorldStateFunctionLibrary.SetWorldStateValue` (make `BHWorldStateValue`) (`self.NullActor`)))
  (return (`|MakeArray` (make `BHWorldStateData` (make `BHWorldStateKey` AgentActor (`self.ObjectHeldWorldStateTag`)) _result))))