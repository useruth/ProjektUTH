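; Enemy gameplay ability and planner action in which an agent reports to a commanding actor and awaits dismissal.
; Planning hooks offer it to clear another actor's WaitForActor world state, requiring the agent to be at that actor and holding nothing.
; On activation it faces that actor, salutes, sends Event.CheckIn and waits for Event.CheckOut.
; Check-out makes it non-cancelable, then a bow montage plays before it ends.
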(event `self.K2_ActivateAbility`
  (bind _returnvalue (`self.GetAvatarActorFromActorInfo`))
  (`self.SetCanBeCanceled` true)
  (`self.K2_CommitAbility`)
  (`Actor.K2_SetActorRotation` (cast `/Game/Blueprints/BP_BHCharacterBase` _returnvalue :!pure true) (`KismetMathLibrary.MakeRotator` 0.0 0.0 (.yaw (`KismetMathLibrary.FindLookAtRotation` (`Actor.K2_GetActorLocation` _returnvalue) (`Actor.K2_GetActorLocation` (`self.InstigatorActor`))))) false)
  (`AbilityTask_PlayMontageAndWait.CreatePlayMontageAndWaitProxy` "None" "/Game/Animations/Salute_Montage.Salute_Montage"
    (:`OnCompleted`
      _)
    (:`OnInterrupted`
      _)
    (:`OnCancelled`
      _))
  (`AbilitySystemBlueprintLibrary.SendGameplayEventToActor` (`self.InstigatorActor`) (struct :`TagName` "Event.CheckIn"))
  (`AbilityTask_WaitGameplayEvent.WaitGameplayEvent` (struct :`TagName` "Event.CheckOut") null
    (:`EventReceived`
      (`self.SetCanBeCanceled` false)
      (`AbilityTask_PlayMontageAndWait.CreatePlayMontageAndWaitProxy` "None" "/Game/Animations/Quick_Formal_Bow_Montage.Quick_Formal_Bow_Montage"
        (:`OnCompleted`
          _)
        (:`OnInterrupted`
          _)
        (:`OnCancelled`
          _))
      (`self.K2_EndAbility`))))

(event `self.K2_OnEndAbility`
  (params (bWasCancelled :type Boolean))
  (`parent.K2_OnEndAbility` bWasCancelled))

(event `self.SetActionTargetData`
  (params (TargetData :type "BHWorldStateData Structure"))
  (set `self.InstigatorActor` (`.WorldStateActor` (break `BHWorldStateKey` (`.WorldStateKey` (break `BHWorldStateData` TargetData))))))

(fn `CanChangeWorldState`
  (params (DesiredWorldState :type "BHWorldStateData Structure") (AgentActor :type "Actor Object Reference"))
  (returns (ReturnValue :type Boolean))
  (bind (_worldstatekey _worldstatevalue) (break `BHWorldStateData` DesiredWorldState))
  (bind (_worldstateactor _worldstatedatatag) (break `BHWorldStateKey` _worldstatekey))
  (if (and (!= _worldstateactor AgentActor) (== _worldstatedatatag (`self.WaitForActorWorldStateTag`)))
    (bind _returnvalue (`BHWorldStateFunctionLibrary.GetWorldStateValueAsActor` _worldstatevalue))
    (return (== _returnvalue (`self.NullActorRef`)))
    (else
      (return false))))

(fn `GetActionCost`
  (params (DesiredWorldState :type "BHWorldStateData Structure") (AgentActor :type "Actor Object Reference"))
  (returns (ReturnValue :type Integer))
  (return (`self.ActionCost`)))

(fn `GetActionEffectWithContextActor`
  (params (AgentActor :type "Actor Object Reference") (TargetActor :type "Actor Object Reference"))
  (returns (EffectWorldState :type "BHWorldStateData Structure") (ReturnValue :type Boolean))
  (locals (LAgent :type "Actor Object Reference") (LTarget :type "Actor Object Reference") (LWorldStateProvider :type "BHWorldStateProvider Object Reference"))
  (set `local.LAgent` AgentActor)
  (set `local.LTarget` TargetActor)
  (bind _output_get (set `local.LWorldStateProvider` (`Actor.GetComponentByClass` (`local.LTarget`) "/Script/BrainHacker.BHWorldStateProvider")))
  (`/Engine/EditorBlueprintResources/StandardMacros.IsValid` _output_get
    (:`Is Valid`
      (bind _returnvalue (`BHWorldStateProvider.HasWorldStateValue` (`local.LWorldStateProvider`) (`self.WaitForActorWorldStateTag`)))
      (if _returnvalue
        (bind _result (`BHWorldStateFunctionLibrary.SetWorldStateValue` (make `BHWorldStateValue`) (`self.NullActorRef`)))
        (return (make `BHWorldStateData` (make `BHWorldStateKey` (`local.LTarget`) (`self.WaitForActorWorldStateTag`)) _result) true)
        (else
          (return (struct) false))))
    (:`Is Not Valid`
      (return (struct) false))))

(fn `GetWorldStatePreconditions`
  (params (ForDesiredWorldState :type "BHWorldStateData Structure") (AgentActor :type "Actor Object Reference"))
  (returns (ReturnValue :type "Array of BHWorldStateData Structure"))
  (bind _result (`BHWorldStateFunctionLibrary.SetWorldStateValue` (make `BHWorldStateValue`) (`.WorldStateActor` (break `BHWorldStateKey` (`.WorldStateKey` (break `BHWorldStateData` ForDesiredWorldState))))))
  (bind _result_2 (`BHWorldStateFunctionLibrary.SetWorldStateValue` (make `BHWorldStateValue`) (`self.NullActorRef`)))
  (return (`|MakeArray` (make `BHWorldStateData` (make `BHWorldStateKey` AgentActor (`self.LocationWorldStateTag`)) _result) (make `BHWorldStateData` (make `BHWorldStateKey` AgentActor (`self.ObjectHeldWorldStateTag`)) _result_2))))