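; Enemy gameplay ability that doubles as a planner action, letting an NPC become alerted by taking over memory from an already alerted NPC.
; For planning, it serves the agent's own IsAlerted goal and requires being at the first alerted NPC in its memory with nothing held.
; On activation it faces that NPC and plays a montage, whose "Enable" notify copies remembered playable characters into the agent's memory.
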(event `self.K2_ActivateAbility`
  (bind _returnvalue (`self.GetAvatarActorFromActorInfo`))
  (bind _character (`self.GetFirstAlertedNPC` (cast `/Game/Blueprints/BP_BHNPCCharacterBase` (`self.GetAvatarActorFromActorInfo`) :!pure true)))
  (bind _output_get (set `self.CachedTargetNPC` _character))
  (`/Engine/EditorBlueprintResources/StandardMacros.IsValid` _output_get
    (:`Is Valid`
      (`self.SetCanBeCanceled` false)
      (`self.K2_CommitAbility`)
      (`Actor.K2_SetActorRotation` (cast `/Game/Blueprints/BP_BHCharacterBase` _returnvalue :!pure true) (`KismetMathLibrary.MakeRotator` 0.0 0.0 (.yaw (`KismetMathLibrary.FindLookAtRotation` (`Actor.K2_GetActorLocation` _returnvalue) (`Actor.K2_GetActorLocation` (`self.CachedTargetNPC`))))) false)
      (bind _notifyname (`|PlayMontage` (`Actor.GetComponentByClass` _returnvalue "/Script/Engine.SkeletalMeshComponent") "/Game/Animations/Button_Pushing_Montage.Button_Pushing_Montage")
        (:`OnCompleted`
          (`self.K2_EndAbility` :!label _label))
        (:`OnInterrupted`
          (goto _label))
        (:`OnNotifyBegin`
          (if (== _notifyname "Enable")
            (for _array_element (`BHMemoryComponent.GetMemory` (`/Game/Blueprints/BP_BHNPCCharacterBase.BHMemory` (`self.CachedTargetNPC`)))
              (bind _asbp_bhplayable_character (cast `/Game/Blueprints/BP_BHPlayableCharacter` _array_element))
              (`BHMemoryComponent.RegisterActorInMemory` (`/Game/Blueprints/BP_BHNPCCharacterBase.BHMemory` (cast `/Game/Blueprints/BP_BHNPCCharacterBase` (`self.GetAvatarActorFromActorInfo`) :!pure true)) _asbp_bhplayable_character))))))
    (:`Is Not Valid`
      (`self.K2_CancelAbility`))))

(event `self.K2_OnEndAbility`
  (params (bWasCancelled :type Boolean))
  (`parent.K2_OnEndAbility` bWasCancelled))

(event `self.SetActionTargetData`
  (params (TargetData :type "BHWorldStateData Structure"))
  ;[1 1 1] this ability not need target data
)

(fn `CanChangeWorldState`
  (params (DesiredWorldState :type "BHWorldStateData Structure") (AgentActor :type "Actor Object Reference"))
  (returns (ReturnValue :type Boolean))
  (bind (_worldstatekey _worldstatevalue) (break `BHWorldStateData` DesiredWorldState))
  (bind (_worldstateactor _worldstatedatatag) (break `BHWorldStateKey` _worldstatekey))
  (if (and (== _worldstateactor AgentActor) (== _worldstatedatatag (`self.IsAlertedWorldStateTag`)))
    (bind _returnvalue (`BHWorldStateFunctionLibrary.GetWorldStateValueAsBool` _worldstatevalue))
    (return _returnvalue)
    (else
      (return false))))

(fn `GetActionCost`
  (params (DesiredWorldState :type "BHWorldStateData Structure") (AgentActor :type "Actor Object Reference") (WithCurrentWorldState :type "Array of BHWorldStateData Structure (by ref)"))
  (returns (ReturnValue :type Integer))
  (return (`self.ActionCost`)))

(fn `GetActionEffectWithContextActor`
  (params (AgentActor :type "Actor Object Reference") (TargetActor :type "Actor Object Reference"))
  (returns (EffectWorldState :type "BHWorldStateData Structure") (ReturnValue :type Boolean))
  (locals (LAgent :type "Actor Object Reference") (LTarget :type "Actor Object Reference") (LWorldStateProvider :type "BHWorldStateProvider Object Reference"))
  (set `local.LAgent` AgentActor)
  (set `local.LTarget` TargetActor)
  (bind _output_get (set `local.LWorldStateProvider` (`Actor.GetComponentByClass` (`local.LTarget`) "/Script/BrainHacker.BHWorldStateProvider")))
  (`/Engine/EditorBlueprintResources/StandardMacros.IsValid` _output_get
    (:`Is Valid`
      (bind _returnvalue (`BHWorldStateProvider.HasWorldStateValue` (`local.LWorldStateProvider`) (`self.IsAlertedWorldStateTag`)))
      (if _returnvalue
        (bind _result (`BHWorldStateFunctionLibrary.SetWorldStateValue` (make `BHWorldStateValue`) (`self.WorldStateIsAlertedEffect`)))
        (return (make `BHWorldStateData` (make `BHWorldStateKey` (`local.LTarget`) (`self.IsAlertedWorldStateTag`)) _result) true)
        (else
          (return (struct) false))))
    (:`Is Not Valid`
      (return (struct) false))))

(fn `GetFirstAlertedNPC`
  (params (ForAgent :type "/Game/Blueprints/BP_BHNPCCharacterBase Object Reference"))
  (returns (Character :type "/Game/Blueprints/BP_BHNPCCharacterBase Object Reference"))
  (for _array_element (`BHMemoryComponent.GetMemory` (`/Game/Blueprints/BP_BHNPCCharacterBase.BHMemory` ForAgent))
    (bind _asbp_bhnpccharacter_base (cast `/Game/Blueprints/BP_BHNPCCharacterBase` _array_element))
    (bind _worldstateprovider (`BrainHackerCharacter.WorldStateProvider` _asbp_bhnpccharacter_base))
    (bind _returnvalue (`BHWorldStateProvider.HasWorldStateValue` _worldstateprovider (struct :`TagName` "WorldState.IsAlerted")))
    (if _returnvalue
      (bind _returnvalue_2 (`BHWorldStateProvider.GetWorldStateValue` _worldstateprovider (struct :`TagName` "WorldState.IsAlerted")))
      (bind _returnvalue_3 (`BHWorldStateFunctionLibrary.GetWorldStateValueAsBool` _returnvalue_2))
      (if _returnvalue_3
        (return _asbp_bhnpccharacter_base))))
  (return null))

(fn `GetWorldStatePreconditions`
  (params (ForDesiredWorldState :type "BHWorldStateData Structure") (AgentActor :type "Actor Object Reference"))
  (returns (ReturnValue :type "Array of BHWorldStateData Structure"))
  (bind _character (`self.GetFirstAlertedNPC` (cast `/Game/Blueprints/BP_BHNPCCharacterBase` AgentActor :!pure true)))
  (bind _result (`BHWorldStateFunctionLibrary.SetWorldStateValue` (make `BHWorldStateValue`) _character))
  (bind _result_2 (`BHWorldStateFunctionLibrary.SetWorldStateValue` (make `BHWorldStateValue`) (`self.NullActor`)))
  (return (`|MakeArray` (make `BHWorldStateData` (make `BHWorldStateKey` AgentActor (`self.LocationWorldStateTag`)) _result) (make `BHWorldStateData` (make `BHWorldStateKey` AgentActor (`self.ObjectHeldWorldStateTag`)) _result_2))))