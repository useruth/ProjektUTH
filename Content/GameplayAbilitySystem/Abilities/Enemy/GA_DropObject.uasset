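; Enemy gameplay ability that drops the held object by calling ReleaseObject on the avatar's grab handle component, then ends immediately.
; It doubles as a planner action with a configurable cost, no preconditions and no target data.
; It can satisfy a desired world state where the agent's held-object value is a null actor.
; Its predicted effect clears that value, provided the agent's world state provider has one.
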(event `self.K2_ActivateAbility`
  (`self.SetCanBeCanceled` false)
  (`self.K2_CommitAbility`)
  (`BHObjectGrabHandleComponent.ReleaseObject` (`Actor.GetComponentByClass` (`self.GetAvatarActorFromActorInfo`) "/Script/BrainHacker.BHObjectGrabHandleComponent"))
  (`self.K2_EndAbility`))

(event `self.K2_OnEndAbility`
  (params (bWasCancelled :type Boolean))
  (`parent.K2_OnEndAbility` bWasCancelled))

(event `self.SetActionTargetData`
  (params (TargetData :type "BHWorldStateData Structure"))
  ;[1 1 1] target data not required for this ability
)

(fn `CanChangeWorldState`
  (params (DesiredWorldState :type "BHWorldStateData Structure") (AgentActor :type "Actor Object Reference"))
  (returns (ReturnValue :type Boolean))
  (bind (_worldstatekey _worldstatevalue) (break `BHWorldStateData` DesiredWorldState))
  (bind (_worldstateactor _worldstatedatatag) (break `BHWorldStateKey` _worldstatekey))
  (if (and (== _worldstateactor AgentActor) (== _worldstatedatatag (`self.ObjectHeldWorldStateTag`)))
    (bind _returnvalue (`BHWorldStateFunctionLibrary.IsWorldStateValueOfTypeActor` _worldstatevalue))
    (if _returnvalue
      (bind _returnvalue_2 (`BHWorldStateFunctionLibrary.GetWorldStateValueAsActor` _worldstatevalue))
      (return (== _returnvalue_2 null))
      (else
        (return false)))
    (else
      (return false))))

(fn `GetActionCost`
  (params (DesiredWorldState :type "BHWorldStateData Structure") (AgentActor :type "Actor Object Reference"))
  (returns (ReturnValue :type Integer))
  (return (`self.ActionCost`)))

(fn `GetActionEffectWithContextActor`
  (params (AgentActor :type "Actor Object Reference") (TargetActor :type "Actor Object Reference"))
  (returns (EffectWorldState :type "BHWorldStateData Structure") (ReturnValue :type Boolean))
  (locals (LAgent :type "Actor Object Reference") (LTarget :type "Actor Object Reference") (LWorldStateProvider :type "BHWorldStateProvider Object Reference"))
  (set `local.LAgent` AgentActor)
  (set `local.LTarget` TargetActor)
  (bind _output_get (set `local.LWorldStateProvider` (`Actor.GetComponentByClass` (`local.LAgent`) "/Script/BrainHacker.BHWorldStateProvider")))
  (`/Engine/EditorBlueprintResources/StandardMacros.IsValid` _output_get
    (:`Is Valid`
      (bind _returnvalue (`BHWorldStateProvider.HasWorldStateValue` (`local.LWorldStateProvider`) (`self.ObjectHeldWorldStateTag`)))
      (if _returnvalue
        (bind _result (`BHWorldStateFunctionLibrary.SetWorldStateValue` (make `BHWorldStateValue`) (`self.NullActorRef`)))
        (return (make `BHWorldStateData` (make `BHWorldStateKey` (`local.LAgent`) (`self.ObjectHeldWorldStateTag`)) _result) true)
        (else
          (return (struct) false))))
    (:`Is Not Valid`
      (return (struct) false))))

(fn `GetWorldStatePreconditions`
  (params (ForDesiredWorldState :type "BHWorldStateData Structure") (AgentActor :type "Actor Object Reference"))
  (returns (ReturnValue :type "Array of BHWorldStateData Structure"))
  ;[1 1 1] not preconditions for this ability
  (return (`|MakeArray`)))