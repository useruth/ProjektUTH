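; Enemy gameplay ability that doubles as a planner action for putting a held object into a generator as its battery.
; On activation it turns the avatar toward the target generator and plays a pushing montage, whose Detach notify releases and destroys the held object and sets the generator's battery flag.
; For planning, it advertises the has-battery effect and requires the agent to be at the generator holding its required object.
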(event `self.K2_ActivateAbility`
  (bind _returnvalue (`self.GetAvatarActorFromActorInfo`))
  (bind _returnvalue_2 (`Actor.GetComponentByClass` (cast `/Game/Blueprints/BP_BHCharacterBase` (`self.GetAvatarActorFromActorInfo`) :!pure true) "/Script/BrainHacker.BHObjectGrabHandleComponent"))
  (`self.SetCanBeCanceled` false)
  (`self.K2_CommitAbility`)
  (`Actor.K2_SetActorRotation` (cast `/Game/Blueprints/BP_BHCharacterBase` _returnvalue :!pure true) (`KismetMathLibrary.MakeRotator` 0.0 0.0 (.yaw (`KismetMathLibrary.FindLookAtRotation` (`Actor.K2_GetActorLocation` _returnvalue) (`Actor.K2_GetActorLocation` (`self.TargetInteractionObject`))))) false)
  (bind _notifyname (`|PlayMontage` (`Actor.GetComponentByClass` _returnvalue "/Script/Engine.SkeletalMeshComponent") "/Game/Animations/Pushing_Montage.Pushing_Montage")
    (:`OnCompleted`
      (`self.K2_EndAbility` :!label _label))
    (:`OnInterrupted`
      (goto _label))
    (:`OnNotifyBegin`
      (if (== _notifyname "Detach")
        (bind _returnvalue_3 (`BHObjectGrabHandleComponent.GetCurrentObject` _returnvalue_2))
        (set `self.CachedGrabbableObject` _returnvalue_3)
        (`BHObjectGrabHandleComponent.ReleaseObject` _returnvalue_2)
        (`/Game/Blueprints/BP_Generator.SetGeneratorHasBattery` (`self.TargetInteractionObject`) true)
        (`Actor.K2_DestroyActor` (`self.CachedGrabbableObject`))))))

(event `self.K2_OnEndAbility`
  (params (bWasCancelled :type Boolean))
  (`parent.K2_OnEndAbility` bWasCancelled))

(event `self.SetActionTargetData`
  (params (TargetData :type "BHWorldStateData Structure"))
  (set `self.TargetInteractionObject` (cast `/Game/Blueprints/BP_Generator` (`.WorldStateActor` (break `BHWorldStateKey` (`.WorldStateKey` (break `BHWorldStateData` TargetData)))) :!pure true)))

(fn `CanChangeWorldState`
  (params (DesiredWorldState :type "BHWorldStateData Structure") (AgentActor :type "Actor Object Reference"))
  (returns (ReturnValue :type Boolean))
  (bind (_worldstatekey _worldstatevalue) (break `BHWorldStateData` DesiredWorldState))
  (bind (_worldstateactor _worldstatedatatag) (break `BHWorldStateKey` _worldstatekey))
  (if (and (`.bSuccess` (cast `/Game/Blueprints/BP_Generator` _worldstateactor :!pure true)) (== _worldstatedatatag (`self.HasBatteryWorldStateTag`)))
    (bind _returnvalue (`BHWorldStateFunctionLibrary.GetWorldStateValueAsBool` _worldstatevalue))
    (return _returnvalue)
    (else
      (return false))))

(fn `GetActionCost`
  (params (DesiredWorldState :type "BHWorldStateData Structure") (AgentActor :type "Actor Object Reference"))
  (returns (ReturnValue :type Integer))
  (return (`self.ActionCost`)))

(fn `GetActionEffectWithContextActor`
  (params (AgentActor :type "Actor Object Reference") (TargetActor :type "Actor Object Reference"))
  (returns (EffectWorldState :type "BHWorldStateData Structure") (ReturnValue :type Boolean))
  (locals (LAgent :type "Actor Object Reference") (LTarget :type "Actor Object Reference") (LWorldStateProvider :type "BHWorldStateProvider Object Reference"))
  (set `local.LAgent` AgentActor)
  (set `local.LTarget` TargetActor)
  (bind _output_get (set `local.LWorldStateProvider` (`Actor.GetComponentByClass` (`local.LTarget`) "/Script/BrainHacker.BHWorldStateProvider")))
  (`/Engine/EditorBlueprintResources/StandardMacros.IsValid` _output_get
    (:`Is Valid`
      (bind _returnvalue (`BHWorldStateProvider.HasWorldStateValue` (`local.LWorldStateProvider`) (`self.HasBatteryWorldStateTag`)))
      (if _returnvalue
        (bind _result (`BHWorldStateFunctionLibrary.SetWorldStateValue` (make `BHWorldStateValue`) (`self.WorldStateHasBatteryEffect`)))
        (return (make `BHWorldStateData` (make `BHWorldStateKey` (`local.LTarget`) (`self.HasBatteryWorldStateTag`)) _result) true)
        (else
          (return (struct) false))))
    (:`Is Not Valid`
      (return (struct) false))))

(fn `GetWorldStatePreconditions`
  (params (ForDesiredWorldState :type "BHWorldStateData Structure") (AgentActor :type "Actor Object Reference"))
  (returns (ReturnValue :type "Array of BHWorldStateData Structure"))
  (bind _worldstateactor (break `BHWorldStateKey` (`.WorldStateKey` (break `BHWorldStateData` ForDesiredWorldState))))
  (bind _result (`BHWorldStateFunctionLibrary.SetWorldStateValue` (make `BHWorldStateValue`) _worldstateactor))
  (bind _result_2 (`/Game/Blueprints/BP_Generator.GetRequiredObject` (cast `/Game/Blueprints/BP_Generator` _worldstateactor :!pure true)))
  (bind _result_3 (`BHWorldStateFunctionLibrary.SetWorldStateValue` (make `BHWorldStateValue`) _result_2))
  (return (`|MakeArray` (make `BHWorldStateData` (make `BHWorldStateKey` AgentActor (`self.LocationWorldStateTag`)) _result) (make `BHWorldStateData` (make `BHWorldStateKey` AgentActor (`self.ObjectHeldWorldStateTag`)) _result_3))))