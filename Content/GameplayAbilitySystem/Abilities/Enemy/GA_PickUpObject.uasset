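; Enemy gameplay ability that picks up a grabbable object and doubles as a planner action using world-state preconditions, effects and cost.
; It can satisfy an object-held world state targeting a BHGrabbableObject, requiring the agent to be at that object with nothing held.
; On activation it becomes non-cancelable, turns the avatar toward the target, plays a pickup montage, and grabs via BHObjectGrabHandleComponent on the "Attach" notify.
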(event `self.K2_ActivateAbility`
  (bind _returnvalue (`self.GetAvatarActorFromActorInfo`))
  (`self.SetCanBeCanceled` false)
  (`self.K2_CommitAbility`)
  (`Actor.K2_SetActorRotation` (cast `/Game/Blueprints/BP_BHCharacterBase` _returnvalue :!pure true) (`KismetMathLibrary.MakeRotator` 0.0 0.0 (.yaw (`KismetMathLibrary.FindLookAtRotation` (`Actor.K2_GetActorLocation` _returnvalue) (`Actor.K2_GetActorLocation` (`self.TargetGrabbableObject`))))) false)
  (bind _notifyname (`|PlayMontage` (`Actor.GetComponentByClass` _returnvalue "/Script/Engine.SkeletalMeshComponent") "/Game/Animations/Pickup_Object_Montage.Pickup_Object_Montage")
    (:`OnCompleted`
      (`self.K2_EndAbility` :!label _label))
    (:`OnInterrupted`
      (goto _label))
    (:`OnNotifyBegin`
      (if (== _notifyname "Attach")
        (`BHObjectGrabHandleComponent.GrabObject` (`Actor.GetComponentByClass` (`self.GetAvatarActorFromActorInfo`) "/Script/BrainHacker.BHObjectGrabHandleComponent") (cast `BHGrabbableObject` (`self.TargetGrabbableObject`) :!pure true))))))

(event `self.K2_OnEndAbility`
  (params (bWasCancelled :type Boolean))
  (`parent.K2_OnEndAbility` bWasCancelled))

(event `self.SetActionTargetData`
  (params (TargetData :type "BHWorldStateData Structure"))
  (bind _returnvalue (`BHWorldStateFunctionLibrary.GetWorldStateValueAsActor` (`.WorldStateValue` (break `BHWorldStateData` TargetData))))
  (set `self.TargetGrabbableObject` _returnvalue))

(fn `CanChangeWorldState`
  (params (DesiredWorldState :type "BHWorldStateData Structure") (AgentActor :type "Actor Object Reference"))
  (returns (ReturnValue :type Boolean))
  (bind (_worldstatekey _worldstatevalue) (break `BHWorldStateData` DesiredWorldState))
  (bind (_worldstateactor _worldstatedatatag) (break `BHWorldStateKey` _worldstatekey))
  (if (and (== _worldstateactor AgentActor) (== _worldstatedatatag (`self.ObjectHeldWorldStateTag`)))
    (bind _returnvalue (`BHWorldStateFunctionLibrary.IsWorldStateValueOfTypeActor` _worldstatevalue))
    (if _returnvalue
      (bind _returnvalue_2 (`BHWorldStateFunctionLibrary.GetWorldStateValueAsActor` _worldstatevalue))
      (return (`KismetSystemLibrary.DoesImplementInterface` _returnvalue_2 "/Script/BrainHacker.BHGrabbableObject"))
      (else
        (return false)))
    (else
      (return false))))

(fn `GetActionCost`
  (params (DesiredWorldState :type "BHWorldStateData Structure") (AgentActor :type "Actor Object Reference"))
  (returns (ReturnValue :type Integer))
  (return (`self.ActionCost`)))

(fn `GetActionEffectWithContextActor`
  (params (AgentActor :type "Actor Object Reference") (TargetActor :type "Actor Object Reference"))
  (returns (EffectWorldState :type "BHWorldStateData Structure") (ReturnValue :type Boolean))
  (locals (LAgent :type "Actor Object Reference") (LTarget :type "Actor Object Reference") (LWorldStateProvider :type "BHWorldStateProvider Object Reference"))
  (set `local.LAgent` AgentActor)
  (set `local.LTarget` TargetActor)
  (bind _output_get (set `local.LWorldStateProvider` (`Actor.GetComponentByClass` (`local.LAgent`) "/Script/BrainHacker.BHWorldStateProvider")))
  (`/Engine/EditorBlueprintResources/StandardMacros.IsValid` _output_get
    (:`Is Valid`
      (bind _returnvalue (`BHWorldStateProvider.HasWorldStateValue` (`local.LWorldStateProvider`) (`self.ObjectHeldWorldStateTag`)))
      (if _returnvalue
        (bind _result (`BHWorldStateFunctionLibrary.SetWorldStateValue` (make `BHWorldStateValue`) (`local.LTarget`)))
        (return (make `BHWorldStateData` (make `BHWorldStateKey` (`local.LAgent`) (`self.ObjectHeldWorldStateTag`)) _result) true)
        (else
          (return (struct) false))))
    (:`Is Not Valid`
      (return (struct) false))))

(fn `GetWorldStatePreconditions`
  (params (ForDesiredWorldState :type "BHWorldStateData Structure") (AgentActor :type "Actor Object Reference"))
  (returns (ReturnValue :type "Array of BHWorldStateData Structure"))
  (bind _returnvalue (`BHWorldStateFunctionLibrary.GetWorldStateValueAsActor` (`.WorldStateValue` (break `BHWorldStateData` ForDesiredWorldState))))
  (bind _result (`BHWorldStateFunctionLibrary.SetWorldStateValue` (make `BHWorldStateValue`) _returnvalue))
  (bind _result_2 (`BHWorldStateFunctionLibrary.SetWorldStateValue` (make `BHWorldStateValue`) (`self.NullActorRef`)))
  (return (`|MakeArray` (make `BHWorldStateData` (make `BHWorldStateKey` AgentActor (`self.LocationWorldStateTag`)) _result) (make `BHWorldStateData` (make `BHWorldStateKey` AgentActor (`self.ObjectHeldWorldStateTag`)) _result_2))))