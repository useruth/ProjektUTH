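; Enemy gameplay ability that makes an NPC dance to a YMCA montage, doubling as a planner action that satisfies the agent's own HaveFun world state.
; Activation commits as cancelable, sets HasCharacterFun on the avatar and plays the montage; ending clears the flag.
; Planner overrides report a fixed cost, no preconditions or target data, and offer the HaveFun effect only when the agent's world state provider holds that key.
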(event `self.SetActionTargetData`
  (params (TargetData :type "BHWorldStateData Structure"))
  ;[1 1 1] this ability not need target data
)

(event `self.K2_ActivateAbility`
  (`self.SetCanBeCanceled` true)
  (`self.K2_CommitAbility`)
  (set `/Game/Blueprints/BP_BHNPCCharacterBase.bHasCharacterFun` true (cast `/Game/Blueprints/BP_BHNPCCharacterBase` (`self.GetAvatarActorFromActorInfo`) :!pure true))
  (`AbilityTask_PlayMontageAndWait.CreatePlayMontageAndWaitProxy` "None" "/Game/Animations/Ymca_Dance_Montage.Ymca_Dance_Montage"))

(event `self.K2_OnEndAbility`
  (params (bWasCancelled :type Boolean))
  (set `/Game/Blueprints/BP_BHNPCCharacterBase.bHasCharacterFun` false (cast `/Game/Blueprints/BP_BHNPCCharacterBase` (`self.GetAvatarActorFromActorInfo`) :!pure true))
  (`parent.K2_OnEndAbility` bWasCancelled))

(fn `CanChangeWorldState`
  (params (DesiredWorldState :type "BHWorldStateData Structure") (AgentActor :type "Actor Object Reference"))
  (returns (ReturnValue :type Boolean))
  (bind (_worldstatekey _worldstatevalue) (break `BHWorldStateData` DesiredWorldState))
  (bind (_worldstateactor _worldstatedatatag) (break `BHWorldStateKey` _worldstatekey))
  (if (and (== _worldstateactor AgentActor) (== _worldstatedatatag (`self.HaveFunWorldStateTag`)))
    (bind _returnvalue (`BHWorldStateFunctionLibrary.GetWorldStateValueAsBool` _worldstatevalue))
    (return _returnvalue)
    (else
      (return false))))

(fn `GetActionCost`
  (params (DesiredWorldState :type "BHWorldStateData Structure") (AgentActor :type "Actor Object Reference"))
  (returns (ReturnValue :type Integer))
  (return (`self.ActionCost`)))

(fn `GetActionEffectWithContextActor`
  (params (AgentActor :type "Actor Object Reference") (TargetActor :type "Actor Object Reference"))
  (returns (EffectWorldState :type "BHWorldStateData Structure") (ReturnValue :type Boolean))
  (locals (LAgent :type "Actor Object Reference") (LTarget :type "Actor Object Reference") (LWorldStateProvider :type "BHWorldStateProvider Object Reference"))
  (set `local.LAgent` AgentActor)
  (set `local.LTarget` TargetActor)
  (bind _output_get (set `local.LWorldStateProvider` (`Actor.GetComponentByClass` (`local.LAgent`) "/Script/BrainHacker.BHWorldStateProvider")))
  (`/Engine/EditorBlueprintResources/StandardMacros.IsValid` _output_get
    (:`Is Valid`
      (bind _returnvalue (`BHWorldStateProvider.HasWorldStateValue` (`local.LWorldStateProvider`) (`self.HaveFunWorldStateTag`)))
      (if _returnvalue
        (bind _result (`BHWorldStateFunctionLibrary.SetWorldStateValue` (make `BHWorldStateValue`) (`self.WorldStateHaveFunEffect`)))
        (return (make `BHWorldStateData` (make `BHWorldStateKey` (`local.LAgent`) (`self.HaveFunWorldStateTag`)) _result) true)
        (else
          (return (struct) false))))
    (:`Is Not Valid`
      (return (struct) false))))

(fn `GetWorldStatePreconditions`
  (params (ForDesiredWorldState :type "BHWorldStateData Structure") (AgentActor :type "Actor Object Reference"))
  (returns (ReturnValue :type "Array of BHWorldStateData Structure"))
  ;[1 1 1] this ability has not any preconditions
  (return (`|MakeArray`)))