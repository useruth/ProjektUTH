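; Enemy melee attack gameplay ability that doubles as a GOAP-style planner action for reducing another actor's health to zero.
; Planning functions require the agent at the target's location holding nothing, report a health effect and cost, and receive the attack target.
; On activation it becomes uncancelable, faces the target and plays a punch montage.
; The Hit notify applies set-by-caller GE_Damage if the target is within range and cone.
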(event `self.K2_ActivateAbility`
  (bind _returnvalue (`self.GetAvatarActorFromActorInfo`))
  (`self.SetCanBeCanceled` false)
  (`self.K2_CommitAbility`)
  (`Actor.K2_SetActorRotation` (cast `/Game/Blueprints/BP_BHCharacterBase` _returnvalue :!pure true) (`KismetMathLibrary.MakeRotator` 0.0 0.0 (.yaw (`KismetMathLibrary.FindLookAtRotation` (`Actor.K2_GetActorLocation` _returnvalue) (`Actor.K2_GetActorLocation` (`self.AttackTarget`))))) false)
  (bind _notifyname (`|PlayMontage` (`Actor.GetComponentByClass` _returnvalue "/Script/Engine.SkeletalMeshComponent") "/Game/Animations/Cross_Punch_Montage.Cross_Punch_Montage")
    (:`OnCompleted`
      (`self.K2_EndAbility` :!label _label))
    (:`OnInterrupted`
      (goto _label))
    (:`OnNotifyBegin`
      (if (== _notifyname "Hit")
        (bind _result (`self.CheckIsHit`))
        (if _result
          (bind _returnvalue_2 (`AbilitySystemBlueprintLibrary.AssignTagSetByCallerMagnitude` (`self.MakeOutgoingGameplayEffectSpec` "/Game/GameplayAbilitySystem/Effects/GE_Damage.GE_Damage_C") (struct :`TagName` "Magnitude") -25.0))
          (`self.K2_ApplyGameplayEffectSpecToTarget` _returnvalue_2 (`AbilitySystemBlueprintLibrary.AbilityTargetDataFromActor` (`self.AttackTarget`))))))))

(event `self.K2_OnEndAbility`
  (params (bWasCancelled :type Boolean))
  (`parent.K2_OnEndAbility` bWasCancelled))

(event `self.SetActionTargetData`
  (params (TargetData :type "BHWorldStateData Structure"))
  (set `self.AttackTarget` (`.WorldStateActor` (break `BHWorldStateKey` (`.WorldStateKey` (break `BHWorldStateData` TargetData))))))

(fn `CanChangeWorldState`
  (params (DesiredWorldState :type "BHWorldStateData Structure") (AgentActor :type "Actor Object Reference"))
  (returns (ReturnValue :type Boolean))
  (bind (_worldstatekey _worldstatevalue) (break `BHWorldStateData` DesiredWorldState))
  (bind (_worldstateactor _worldstatedatatag) (break `BHWorldStateKey` _worldstatekey))
  (if (and (!= _worldstateactor AgentActor) (== _worldstatedatatag (`self.HealthWorldStateTag`)))
    (bind _returnvalue (`BHWorldStateFunctionLibrary.GetWorldStateValueAsFloat` _worldstatevalue))
    (return (`KismetMathLibrary.NearlyEqual_FloatFloat` _returnvalue))
    (else
      (return false))))

(fn `CheckIsHit`
  (returns (Result :type Boolean))
  (bind _returnvalue (`self.GetAvatarActorFromActorInfo`))
  (if (>= (`self.AttackRange`) (`KismetMathLibrary.Vector_Distance` (`Actor.K2_GetActorLocation` (`self.GetAvatarActorFromActorInfo`)) (`Actor.K2_GetActorLocation` (`self.AttackTarget`))))
    (return (<= (`KismetMathLibrary.DegAcos` (`KismetMathLibrary.Dot_VectorVector` (`Actor.GetActorForwardVector` _returnvalue) (`KismetMathLibrary.Normal` (- (`Actor.K2_GetActorLocation` (`self.AttackTarget`)) (`Actor.K2_GetActorLocation` _returnvalue))))) (`self.AttackCone`)))
    (else
      (return false))))

(fn `GetActionCost`
  (params (DesiredWorldState :type "BHWorldStateData Structure") (AgentActor :type "Actor Object Reference"))
  (returns (ReturnValue :type Integer))
  (return (`self.ActionCost`)))

(fn `GetActionEffectWithContextActor`
  (params (AgentActor :type "Actor Object Reference") (TargetActor :type "Actor Object Reference"))
  (returns (EffectWorldState :type "BHWorldStateData Structure") (ReturnValue :type Boolean))
  (locals (LAgent :type "Actor Object Reference") (LTarget :type "Actor Object Reference") (LWorldStateProvider :type "BHWorldStateProvider Object Reference") (LEffectWorldStateValue :type "BHWorldStateValue Structure"))
  (set `local.LAgent` AgentActor)
  (set `local.LTarget` TargetActor)
  (bind _output_get (set `local.LWorldStateProvider` (`Actor.GetComponentByClass` (`local.LTarget`) "/Script/BrainHacker.BHWorldStateProvider")))
  (`/Engine/EditorBlueprintResources/StandardMacros.IsValid` _output_get
    (:`Is Valid`
      (bind _returnvalue (`BHWorldStateProvider.HasWorldStateValue` (`local.LWorldStateProvider`) (`self.HealthWorldStateTag`)))
      (if _returnvalue
        (bind _result (`BHWorldStateFunctionLibrary.SetWorldStateValue` (make `BHWorldStateValue`) (`self.WorldStateHealthEffect`)))
        (return (make `BHWorldStateData` (make `BHWorldStateKey` (`local.LTarget`) (`self.HealthWorldStateTag`)) _result) true)
        (else
          (return (struct) false))))
    (:`Is Not Valid`
      (return (struct) false))))

(fn `GetWorldStatePreconditions`
  (params (ForDesiredWorldState :type "BHWorldStateData Structure") (AgentActor :type "Actor Object Reference"))
  (returns (ReturnValue :type "Array of BHWorldStateData Structure"))
  (bind _result (`BHWorldStateFunctionLibrary.SetWorldStateValue` (make `BHWorldStateValue`) (`.WorldStateActor` (break `BHWorldStateKey` (`.WorldStateKey` (break `BHWorldStateData` ForDesiredWorldState))))))
  (bind _result_2 (`BHWorldStateFunctionLibrary.SetWorldStateValue` (make `BHWorldStateValue`) (`self.NullActorRef`)))
  (return (`|MakeArray` (make `BHWorldStateData` (make `BHWorldStateKey` AgentActor (`self.LocationWorldStateTag`)) _result) (make `BHWorldStateData` (make `BHWorldStateKey` AgentActor (`self.ObjectHeldWorldStateTag`)) _result_2))))