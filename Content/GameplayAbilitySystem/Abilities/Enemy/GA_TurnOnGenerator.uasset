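; Enemy gameplay ability that doubles as a planner action, switching on the first inactive generator linked to a target energy storage.
; It offers itself for energy-level goals of 1.0, requiring the agent at that generator with empty hands and a desired battery state, and reports an energy-level effect.
; On activation it becomes non-cancelable, faces the generator and plays a button-pushing montage, whose "Enable" notify activates the generator.
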(event `self.K2_ActivateAbility`
  (bind _returnvalue (`self.GetAvatarActorFromActorInfo`))
  (`self.SetCanBeCanceled` false)
  (`self.K2_CommitAbility`)
  (bind _generator (`self.GetFirstDisabledGenerator` (`self.TargetInteractionObject`)))
  (set `self.CachedGeneratorGenerator` _generator)
  (`Actor.K2_SetActorRotation` (cast `/Game/Blueprints/BP_BHCharacterBase` _returnvalue :!pure true) (`KismetMathLibrary.MakeRotator` 0.0 0.0 (.yaw (`KismetMathLibrary.FindLookAtRotation` (`Actor.K2_GetActorLocation` _returnvalue) (`Actor.K2_GetActorLocation` (`self.CachedGeneratorGenerator`))))) false)
  (bind _notifyname (`|PlayMontage` (`Actor.GetComponentByClass` _returnvalue "/Script/Engine.SkeletalMeshComponent") "/Game/Animations/Button_Pushing_Montage.Button_Pushing_Montage")
    (:`OnCompleted`
      (`self.K2_EndAbility` :!label _label))
    (:`OnInterrupted`
      (goto _label))
    (:`OnNotifyBegin`
      (if (== _notifyname "Enable")
        (`/Game/Blueprints/BPI_ActivityObject.SetIsActive` (`self.CachedGeneratorGenerator`) true)))))

(event `self.K2_OnEndAbility`
  (params (bWasCancelled :type Boolean))
  (`parent.K2_OnEndAbility` bWasCancelled))

(event `self.SetActionTargetData`
  (params (TargetData :type "BHWorldStateData Structure"))
  (set `self.TargetInteractionObject` (cast `/Game/Blueprints/BP_EnergyStorage` (`.WorldStateActor` (break `BHWorldStateKey` (`.WorldStateKey` (break `BHWorldStateData` TargetData)))) :!pure true)))

(fn `CanChangeWorldState`
  (params (DesiredWorldState :type "BHWorldStateData Structure") (AgentActor :type "Actor Object Reference"))
  (returns (ReturnValue :type Boolean))
  (bind (_worldstatekey _worldstatevalue) (break `BHWorldStateData` DesiredWorldState))
  (bind (_worldstateactor _worldstatedatatag) (break `BHWorldStateKey` _worldstatekey))
  (if (and (`.bSuccess` (cast `/Game/Blueprints/BP_EnergyStorage` _worldstateactor :!pure true)) (== _worldstatedatatag (`self.EnergyLevelWorldStateTag`)))
    (bind _returnvalue (`BHWorldStateFunctionLibrary.GetWorldStateValueAsFloat` _worldstatevalue))
    (return (`KismetMathLibrary.NearlyEqual_FloatFloat` _returnvalue 1.0))
    (else
      (return false))))

(fn `GetActionCost`
  (params (DesiredWorldState :type "BHWorldStateData Structure") (AgentActor :type "Actor Object Reference"))
  (returns (ReturnValue :type Integer))
  (return (`self.ActionCost`)))

(fn `GetActionEffectWithContextActor`
  (params (AgentActor :type "Actor Object Reference") (TargetActor :type "Actor Object Reference"))
  (returns (EffectWorldState :type "BHWorldStateData Structure") (ReturnValue :type Boolean))
  (locals (LAgent :type "Actor Object Reference") (LTarget :type "Actor Object Reference") (LWorldStateProvider :type "BHWorldStateProvider Object Reference"))
  (set `local.LAgent` AgentActor)
  (set `local.LTarget` TargetActor)
  (bind _output_get (set `local.LWorldStateProvider` (`Actor.GetComponentByClass` (`local.LTarget`) "/Script/BrainHacker.BHWorldStateProvider")))
  (`/Engine/EditorBlueprintResources/StandardMacros.IsValid` _output_get
    (:`Is Valid`
      (bind _returnvalue (`BHWorldStateProvider.HasWorldStateValue` (`local.LWorldStateProvider`) (`self.EnergyLevelWorldStateTag`)))
      (if _returnvalue
        (bind _result (`BHWorldStateFunctionLibrary.SetWorldStateValue` (make `BHWorldStateValue`) (`self.WorldStateEnergyLevelEffect`)))
        (return (make `BHWorldStateData` (make `BHWorldStateKey` (`local.LTarget`) (`self.EnergyLevelWorldStateTag`)) _result) true)
        (else
          (return (struct) false))))
    (:`Is Not Valid`
      (return (struct) false))))

(fn `GetFirstDisabledGenerator`
  (params (ForEnergyStorage :type "/Game/Blueprints/BP_EnergyStorage Object Reference"))
  (returns (Generator :type "/Game/Blueprints/BP_Generator Object Reference"))
  (for _array_element (`/Game/Blueprints/BP_EnergyStorage.PowerGenerators` ForEnergyStorage)
    (bind _result (`/Game/Blueprints/BPI_ActivityObject.GetIsActive` _array_element))
    (if (not _result)
      (return _array_element)))
  (return null))

(fn `GetWorldStatePreconditions`
  (params (ForDesiredWorldState :type "BHWorldStateData Structure") (AgentActor :type "Actor Object Reference"))
  (returns (ReturnValue :type "Array of BHWorldStateData Structure"))
  (bind _generator (`self.GetFirstDisabledGenerator` (cast `/Game/Blueprints/BP_EnergyStorage` (`.WorldStateActor` (break `BHWorldStateKey` (`.WorldStateKey` (break `BHWorldStateData` ForDesiredWorldState)))) :!pure true)))
  (bind _result (`BHWorldStateFunctionLibrary.SetWorldStateValue` (make `BHWorldStateValue`) _generator))
  (bind _result_2 (`BHWorldStateFunctionLibrary.SetWorldStateValue` (make `BHWorldStateValue`) (`self.NullActor`)))
  (bind _result_3 (`BHWorldStateFunctionLibrary.SetWorldStateValue` (make `BHWorldStateValue`) (`self.HasBatteryDesiredState`)))
  (return (`|MakeArray` (make `BHWorldStateData` (make `BHWorldStateKey` AgentActor (`self.LocationWorldStateTag`)) _result) (make `BHWorldStateData` (make `BHWorldStateKey` AgentActor (`self.ObjectHeldWorldStateTag`)) _result_2) (make `BHWorldStateData` (make `BHWorldStateKey` _generator (`self.HasBatteryWorldStateTag`)) _result_3))))