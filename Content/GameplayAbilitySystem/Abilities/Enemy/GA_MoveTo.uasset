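; Enemy GAS ability that serves as a GOAP move-to action, changing the agent's location world state to a target actor or vector.
; For planning, it has no preconditions and costs actions by navmesh path length times a per-meter cost.
; On activation it picks run or walk from the pursued goal's score, then runs AIMoveTo.
; Ending stops movement manually, since AIMoveTo is not a GAS task.
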(event `self.SetActionTargetData`
  (params (TargetData :type "BHWorldStateData Structure"))
  (bind (_worldstatekey _worldstatevalue) (break `BHWorldStateData` TargetData))
  (bind _returnvalue (`BHWorldStateFunctionLibrary.IsWorldStateValueOfTypeActor` _worldstatevalue))
  (if _returnvalue
    (bind _returnvalue_2 (`BHWorldStateFunctionLibrary.GetWorldStateValueAsActor` _worldstatevalue))
    (set `self.TargetActor` _returnvalue_2)
    (set `self.TargetLocation` (0.0 0.0 0.0))
    (else
      (bind _returnvalue_3 (`BHWorldStateFunctionLibrary.GetWorldStateValueAsVector` _worldstatevalue))
      (set `self.TargetLocation` _returnvalue_3)
      (set `self.TargetActor` null))))

(event `self.K2_ActivateAbility`
  (`self.SetCanBeCanceled` true)
  (`self.K2_CommitAbility`)
  (`self.AdjustMovementSpeedToGoalImportance`)
  (`|AIMoveTo` (cast `/Game/Blueprints/BP_BHCharacterBase` (`self.GetAvatarActorFromActorInfo`) :!pure true) (`self.TargetLocation`) (`self.TargetActor`) 100.0
    (:`OnSuccess`
      (`self.K2_EndAbility`))
    (:`OnFail`
      (`self.K2_CancelAbility`))))

(event `self.K2_OnEndAbility`
  (params (bWasCancelled :type Boolean))
  ;[1 1 1] if cancel ability from outside need stop movement (AIMoveTo is not GAS task)
  (`NavMovementComponent.StopActiveMovement` (`Character.CharacterMovement` (cast `/Game/Blueprints/BP_BHCharacterBase` (`self.GetAvatarActorFromActorInfo`) :!pure true)))
  (`parent.K2_OnEndAbility` bWasCancelled))

(fn `AdjustMovementSpeedToGoalImportance`
  (bind _returnvalue (message `BHGOAPAgent.GetGOAPPlanner` (cast `/Game/Blueprints/BP_BHCharacterBase` (`self.GetAvatarActorFromActorInfo`) :!pure true)))
  (bind _returnvalue_2 (`BHGoal.GetGoalScore` (`BHPlanner.GetPursuedGoal` _returnvalue)))
  (bind _asbhcharacter_movement_component (cast `BHCharacterMovementComponent` (`Character.CharacterMovement` (cast `/Game/Blueprints/BP_BHCharacterBase` (`self.GetAvatarActorFromActorInfo`) :!pure true))))
  (`BHCharacterMovementComponent.SetBHMovementMode` _asbhcharacter_movement_component (select `bool` (>= _returnvalue_2 (`self.MinGoalScoreForRunMode`)) :`false` "Walk" :`true` "Run" :!type "EBHMovementMode Enum")))

(fn `CanChangeWorldState`
  (params (DesiredWorldState :type "BHWorldStateData Structure") (AgentActor :type "Actor Object Reference"))
  (returns (ReturnValue :type Boolean))
  (bind (_worldstateactor _worldstatedatatag) (break `BHWorldStateKey` (`.WorldStateKey` (break `BHWorldStateData` DesiredWorldState))))
  (return (and (== _worldstateactor AgentActor) (== _worldstatedatatag (`self.LocationWorldStateTag`)))))

(fn `GetActionCost`
  (params (DesiredWorldState :type "BHWorldStateData Structure") (AgentActor :type "Actor Object Reference") (WithCurrentWorldState :type "Array of BHWorldStateData Structure (by ref)"))
  (returns (ReturnValue :type Integer))
  (locals (LPathLength :type "Float (double-precision)" :default 0.0) (LStartLocation :type "Vector Structure" :default (0.0 0.0 0.0)) (LTargetLocation :type "Vector Structure" :default (0.0 0.0 0.0)))
  (bind (_worldstatekey _worldstatevalue) (break `BHWorldStateData` DesiredWorldState))
  (`|ExecutionSequence`
    (:`then_0`
      ;[1 1 1] find start location
      (bind _returnvalue (`BHWorldStateFunctionLibrary.GetActualWorldStateValue` _worldstatekey WithCurrentWorldState))
      (bind _returnvalue_2 (`BHWorldStateFunctionLibrary.IsWorldStateValueOfTypeVector` _returnvalue))
      (if _returnvalue_2
        (bind _returnvalue_3 (`BHWorldStateFunctionLibrary.GetWorldStateValueAsVector` _returnvalue))
        (set `local.LStartLocation` _returnvalue_3)
        (else
          (bind _returnvalue_4 (`BHWorldStateFunctionLibrary.GetWorldStateValueAsActor` _returnvalue))
          (set `local.LStartLocation` (`Actor.K2_GetActorLocation` _returnvalue_4)))))
    (:`then_1`
      ;[1 1 1] find end location
      (bind _returnvalue_5 (`BHWorldStateFunctionLibrary.IsWorldStateValueOfTypeVector` _worldstatevalue))
      (if _returnvalue_5
        (bind _returnvalue_6 (`BHWorldStateFunctionLibrary.GetWorldStateValueAsVector` _worldstatevalue))
        (set `local.LTargetLocation` _returnvalue_6)
        (else
          (bind _returnvalue_7 (`BHWorldStateFunctionLibrary.GetWorldStateValueAsActor` _worldstatevalue))
          (set `local.LTargetLocation` (`Actor.K2_GetActorLocation` _returnvalue_7)))))
    (:`then_2`
      ;[1 1 1] caclulate cost
      (bind _returnvalue_8 (`NavigationSystemV1.FindPathToLocationSynchronously` (`local.LStartLocation`) (`local.LTargetLocation`) null null))
      (set `local.LPathLength` (`NavigationPath.GetPathLength` _returnvalue_8))
      (return (* (`KismetMathLibrary.FCeil` (/ (`local.LPathLength`) 100.0)) (`self.ActionCostPerMeter`))))))

(fn `GetActionEffectWithContextActor`
  (params (AgentActor :type "Actor Object Reference") (TargetActor :type "Actor Object Reference"))
  (returns (EffectWorldState :type "BHWorldStateData Structure") (ReturnValue :type Boolean))
  (locals (LAgent :type "Actor Object Reference") (LTarget :type "Actor Object Reference") (LWorldStateProvider :type "BHWorldStateProvider Object Reference"))
  (set `local.LAgent` AgentActor)
  (set `local.LTarget` TargetActor)
  (bind _output_get (set `local.LWorldStateProvider` (`Actor.GetComponentByClass` (`local.LTarget`) "/Script/BrainHacker.BHWorldStateProvider")))
  (`/Engine/EditorBlueprintResources/StandardMacros.IsValid` _output_get
    (:`Is Valid`
      (bind _returnvalue (`BHWorldStateProvider.HasWorldStateValue` (`local.LWorldStateProvider`) (`self.LocationWorldStateTag`)))
      (if _returnvalue
        (bind _result (`BHWorldStateFunctionLibrary.SetWorldStateValue` (make `BHWorldStateValue`) (`local.LTarget`)))
        (return (make `BHWorldStateData` (make `BHWorldStateKey` (`local.LAgent`) (`self.LocationWorldStateTag`)) _result) true)
        (else
          (return (struct) false))))
    (:`Is Not Valid`
      (return (struct) false))))

(fn `GetWorldStatePreconditions`
  (params (ForDesiredWorldState :type "BHWorldStateData Structure") (AgentActor :type "Actor Object Reference"))
  (returns (ReturnValue :type "Array of BHWorldStateData Structure"))
  ;[1 1 1] this ability has not any preconditions
  (return (`|MakeArray`)))