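; Enemy GAS ability that doubles as a planner action for programming at a BP_Computer.
; Its planning functions advertise a computer activity effect, requiring the agent to be at the computer, its energy source at a desired level and nothing held.
; On activation the agent faces the computer, plays a typing montage and sets it active.
; An energy source delegate cancels the ability on power loss, and ending deactivates the computer.
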(event `self.K2_ActivateAbility`
  (bind _returnvalue (`self.GetAvatarActorFromActorInfo`))
  (`self.SetCanBeCanceled` true)
  (`self.K2_CommitAbility`)
  (`Actor.K2_SetActorRotation` (cast `/Game/Blueprints/BP_BHCharacterBase` _returnvalue :!pure true) (`KismetMathLibrary.MakeRotator` 0.0 0.0 (.yaw (`KismetMathLibrary.FindLookAtRotation` (`Actor.K2_GetActorLocation` _returnvalue) (`Actor.K2_GetActorLocation` (`self.TargetInteractionObject`))))) false)
  (`AbilityTask_PlayMontageAndWait.CreatePlayMontageAndWaitProxy` "None" "/Game/Animations/Typing_Montage.Typing_Montage"
    (:`then`
      (add `/Game/Blueprints/BP_EnergyStorage.EnergyStorageStateChangedED` (`/Game/Blueprints/BP_Computer.EnergySource` (`self.TargetInteractionObject`)) (`|CreateDelegate` :!event `EnergyStorageStateChanged`))
      (`/Game/Blueprints/BPI_ActivityObject.SetIsActive` (`self.TargetInteractionObject`) true))))

(event `EnergyStorageStateChanged`
  (params (Active :type Boolean))
  (if (not Active)
    (`self.K2_CancelAbility`)))

(event `self.K2_OnEndAbility`
  (params (bWasCancelled :type Boolean))
  (remove `/Game/Blueprints/BP_EnergyStorage.EnergyStorageStateChangedED` (`/Game/Blueprints/BP_Computer.EnergySource` (`self.TargetInteractionObject`)) (`|CreateDelegate` :!event `EnergyStorageStateChanged`))
  (`/Game/Blueprints/BPI_ActivityObject.SetIsActive` (`self.TargetInteractionObject`) false)
  (`parent.K2_OnEndAbility` bWasCancelled))

(event `self.SetActionTargetData`
  (params (TargetData :type "BHWorldStateData Structure"))
  (set `self.TargetInteractionObject` (cast `/Game/Blueprints/BP_Computer` (`.WorldStateActor` (break `BHWorldStateKey` (`.WorldStateKey` (break `BHWorldStateData` TargetData)))) :!pure true)))

(fn `CanChangeWorldState`
  (params (DesiredWorldState :type "BHWorldStateData Structure") (AgentActor :type "Actor Object Reference"))
  (returns (ReturnValue :type Boolean))
  (bind (_worldstatekey _worldstatevalue) (break `BHWorldStateData` DesiredWorldState))
  (bind (_worldstateactor _worldstatedatatag) (break `BHWorldStateKey` _worldstatekey))
  (if (and (`.bSuccess` (cast `/Game/Blueprints/BP_Computer` _worldstateactor :!pure true)) (== _worldstatedatatag (`self.ActivityWorldStateTag`)))
    (bind _returnvalue (`BHWorldStateFunctionLibrary.GetWorldStateValueAsBool` _worldstatevalue))
    (return _returnvalue)
    (else
      (return false))))

(fn `GetActionCost`
  (params (DesiredWorldState :type "BHWorldStateData Structure") (AgentActor :type "Actor Object Reference"))
  (returns (ReturnValue :type Integer))
  (return (`self.ActionCost`)))

(fn `GetActionEffectWithContextActor`
  (params (AgentActor :type "Actor Object Reference") (TargetActor :type "Actor Object Reference"))
  (returns (EffectWorldState :type "BHWorldStateData Structure") (ReturnValue :type Boolean))
  (locals (LAgent :type "Actor Object Reference") (LTarget :type "Actor Object Reference") (LWorldStateProvider :type "BHWorldStateProvider Object Reference"))
  (set `local.LAgent` AgentActor)
  (set `local.LTarget` TargetActor)
  (bind _output_get (set `local.LWorldStateProvider` (`Actor.GetComponentByClass` (`local.LTarget`) "/Script/BrainHacker.BHWorldStateProvider")))
  (`/Engine/EditorBlueprintResources/StandardMacros.IsValid` _output_get
    (:`Is Valid`
      (cast `/Game/Blueprints/BP_Computer` (`local.LTarget`)
        (:`then`
          (bind _returnvalue (`BHWorldStateProvider.HasWorldStateValue` (`local.LWorldStateProvider`) (`self.ActivityWorldStateTag`)))
          (if _returnvalue
            (bind _result (`BHWorldStateFunctionLibrary.SetWorldStateValue` (make `BHWorldStateValue`) (`self.WorldStateActivityEffect`)))
            (return (make `BHWorldStateData` (make `BHWorldStateKey` (`local.LTarget`) (`self.ActivityWorldStateTag`)) _result) true)
            (else
              (return (struct) false))))
        (:`CastFailed`
          (return (struct) false))))
    (:`Is Not Valid`
      (return (struct) false))))

(fn `GetWorldStatePreconditions`
  (params (ForDesiredWorldState :type "BHWorldStateData Structure") (AgentActor :type "Actor Object Reference"))
  (returns (ReturnValue :type "Array of BHWorldStateData Structure"))
  (bind _worldstateactor (break `BHWorldStateKey` (`.WorldStateKey` (break `BHWorldStateData` ForDesiredWorldState))))
  (bind _result (`BHWorldStateFunctionLibrary.SetWorldStateValue` (make `BHWorldStateValue`) _worldstateactor))
  (bind _energystorage (`/Game/Blueprints/BP_Computer.GetEnergySource` (cast `/Game/Blueprints/BP_Computer` _worldstateactor :!pure true)))
  (bind _result_2 (`BHWorldStateFunctionLibrary.SetWorldStateValue` (make `BHWorldStateValue`) (`self.DesiredEnergyLevel`)))
  (bind _result_3 (`BHWorldStateFunctionLibrary.SetWorldStateValue` (make `BHWorldStateValue`) (`self.NullActorRef`)))
  (return (`|MakeArray` (make `BHWorldStateData` (make `BHWorldStateKey` AgentActor (`self.LocationWorldStateTag`)) _result) (make `BHWorldStateData` (make `BHWorldStateKey` _energystorage (`self.EnergyLevelWorldStateTag`)) _result_2) (make `BHWorldStateData` (make `BHWorldStateKey` AgentActor (`self.ObjectHeldWorldStateTag`)) _result_3))))