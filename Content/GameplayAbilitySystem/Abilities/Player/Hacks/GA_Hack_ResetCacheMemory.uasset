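; Player hack ability that makes a targeted NPC forget the player by removing them from its memory.
; Activation requires the targeting component's selected target to be an NPC with an exploit installed that has the ability's owner actor in its BHMemory.
; When hacking finishes, it unregisters the avatar actor from the cached target's BHMemory, then calls the parent hack's finish logic.
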(event `self.HackingFinished`
  (`BHMemoryComponent.UnregisterActorFromMemory` (`/Game/Blueprints/BP_BHNPCCharacterBase.BHMemory` (`self.CachedTarget`)) (`self.GetAvatarActorFromActorInfo`))
  (`parent.HackingFinished`))

(fn `K2_CanActivateAbility`
  (params (ActorInfo :type "GameplayAbilityActorInfo Structure") (Handle :type "GameplayAbilitySpecHandle Structure"))
  (returns (RelevantTags :type "GameplayTagContainer Structure") (ReturnValue :type Boolean))
  (bind (_owneractor _avataractor) (break `GameplayAbilityActorInfo` ActorInfo))
  (bind _asbp_bhnpccharacter_base (cast `/Game/Blueprints/BP_BHNPCCharacterBase` (`BHTargetingComponent.GetSelectedTarget` (`/Game/Blueprints/BP_BHPlayableCharacter.BP_BHTargetingComponent` (cast `/Game/Blueprints/BP_BHPlayableCharacter` _avataractor :!pure true))))
    (:`then`
      (if (`/Game/Blueprints/BP_BHNPCCharacterBase.bIsExploitInstalled` _asbp_bhnpccharacter_base)
        (return (struct) (`BHMemoryComponent.IsActorInMemory` (`/Game/Blueprints/BP_BHNPCCharacterBase.BHMemory` _asbp_bhnpccharacter_base) _owneractor))
        (else
          _)))
    (:`CastFailed`
      _))
  (return (struct) false))