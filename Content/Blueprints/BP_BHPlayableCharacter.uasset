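; BP_BHPlayableCharacter is the player character Blueprint that handles input for choosing and using hacks on targets.
; Next and previous inputs cycle the selected hack in the targeting component.
; On use, with a valid target, it checks the Ability System Component, then sends itself a gameplay event with the hack's trigger tag and target.
; If activation is blocked, the target's enemy panel widget shows a fail indication.
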(event `InputAction|NextHack`
  (params (Key :type "Key Structure"))
  ;[1 1 1] change selected hack
  (:`Pressed`
    (`BHTargetingComponent.SelectNextHack` (`self.BP_BHTargetingComponent`))))

(event `InputAction|PreviousHack`
  (params (Key :type "Key Structure"))
  ;[1 1 1] change selected hack
  (:`Pressed`
    (`BHTargetingComponent.SelectPreviousHack` (`self.BP_BHTargetingComponent`))))

(event `InputAction|UseHack`
  (params (Key :type "Key Structure"))
  ;[1 1 1] activating hacks
  (:`Pressed`
    (`/Engine/EditorBlueprintResources/StandardMacros.IsValid` (`BHTargetingComponent.GetSelectedTarget` (`self.BP_BHTargetingComponent`))
      (:`Is Valid`
        (bind _returnvalue (`BHAbilitySystemComponent.CanActivateAbilityClass` (`self.AbilitySystemComponent`) (`GameplayStatics.GetObjectClass` (`BHTargetingComponent.GetSelectedHack` (`self.BP_BHTargetingComponent`)))))
        (if _returnvalue
          (bind _returnvalue_2 (`BHGameplayAbility.GetTriggerTag` (`BHTargetingComponent.GetSelectedHack` (`self.BP_BHTargetingComponent`))))
          (`AbilitySystemBlueprintLibrary.SendGameplayEventToActor` self _returnvalue_2 (make `GameplayEventData` _returnvalue_2 self (`BHTargetingComponent.GetSelectedTarget` (`self.BP_BHTargetingComponent`))))
          (else
            (`/Game/Widgets/WBP_HackTargetIndicator.ShowFailIndication` (`/Game/Widgets/WBP_EnemyPanel.HackTargetIndicator` (cast `/Game/Widgets/WBP_EnemyPanel` (`WidgetComponent.GetUserWidgetObject` (`/Game/Blueprints/BP_BHNPCCharacterBase.EnemyPanel` (cast `/Game/Blueprints/BP_BHNPCCharacterBase` (`BHTargetingComponent.GetSelectedTarget` (`self.BP_BHTargetingComponent`)) :!pure true))) :!pure true)))))))))

(fn `UserConstructionScript`
  (`parent.UserConstructionScript`))