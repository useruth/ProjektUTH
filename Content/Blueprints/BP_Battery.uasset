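; BP_Battery is a grabbable battery actor that can be picked up and released.
; OnGrab sets the IsGrabbed flag and turns off actor collision and static mesh physics simulation, and OnRelease reverses all three.
; CanBeGrabbed and CanBeReleased derive from that flag, so it can be grabbed only when free and released only when held.
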(event `self.OnRelease`
  (params (Instigator :type "BHObjectGrabHandleComponent Object Reference"))
  (set `self.IsGrabbed` false)
  (`self.SetActorEnableCollision` true)
  (`PrimitiveComponent.SetSimulatePhysics` (`self.StaticMesh`) true))

(event `self.OnGrab`
  (params (Instigator :type "BHObjectGrabHandleComponent Object Reference"))
  (set `self.IsGrabbed` true)
  (`self.SetActorEnableCollision` false)
  (`PrimitiveComponent.SetSimulatePhysics` (`self.StaticMesh`) false))

(fn `CanBeGrabbed`
  (returns (ReturnValue :type Boolean))
  (return (not (`self.IsGrabbed`))))

(fn `CanBeReleased`
  (returns (ReturnValue :type Boolean))
  (return (`self.IsGrabbed`)))

(fn `UserConstructionScript`)