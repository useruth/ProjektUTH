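; BP_Computer is a computer actor that can be switched on or off and draws energy while working.
; SetIsActive sets the working flag, and while it is set, Tick calls ConsumeEnergy on its EnergySource, scaled by EnergyConsumption and frame time.
; Getters expose the active state, the energy source and the world position of an InteractionLocation component.
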(event `/Game/Blueprints/BPI_ActivityObject.SetIsActive`
  (params (Active :type Boolean))
  (set `self.IsComputerWorking` Active))

(event `self.ReceiveTick`
  (params (DeltaSeconds :type "Float (single-precision)"))
  (`parent.ReceiveTick` DeltaSeconds)
  (if (`self.IsComputerWorking`)
    (`/Game/Blueprints/BP_EnergyStorage.ConsumeEnergy` (`self.EnergySource`) (* DeltaSeconds (`self.EnergyConsumption`)))))

(fn `GetEnergySource`
  (returns (EnergyStorage :type "/Game/Blueprints/BP_EnergyStorage Object Reference"))
  (return (`self.EnergySource`)))

(fn `GetInteractionLocation`
  (returns (Result :type "Vector Structure"))
  (return (`SceneComponent.K2_GetComponentLocation` (`self.InteractionLocation`))))

(fn `GetIsActive`
  (returns (Result :type Boolean))
  (return (`self.IsComputerWorking`)))

(fn `UserConstructionScript`)