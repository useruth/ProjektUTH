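; GOAP goal that drives an AI agent to stay alive when threatened.
; An enemy is the nearest playable character in the agent's GOAP memory with a positive attribute value.
; The desired world state targets Fear when an enemy is found, otherwise Health.
; The always-valid goal scores all-or-nothing, firing only with an enemy present and either lost health or fear above half, both read from the Ability System.
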(event `self.UpdateDesiredWorldState`
  (bind _found (`self.GetClosestEnemy` (`self.AgentActor`)))
  (if _found
    (bind _result (`BHWorldStateFunctionLibrary.SetWorldStateValue` (`.WorldStateValue` (break `BHWorldStateData` (`self.DesiredWorldState`))) (`self.DesiredFearWorldState`)))
    (set `self.DesiredWorldState` (make `BHWorldStateData` (make `BHWorldStateKey` (cast `Actor` (`self.AgentActor`) :!pure true) (struct :`TagName` "WorldState.Fear")) _result))
    (else
      (bind _result_2 (`BHWorldStateFunctionLibrary.SetWorldStateValue` (`.WorldStateValue` (break `BHWorldStateData` (`self.DesiredWorldState`))) (`self.DesiredHealthWorldState`)))
      (set `self.DesiredWorldState` (make `BHWorldStateData` (make `BHWorldStateKey` (cast `Actor` (`self.AgentActor`) :!pure true) (struct :`TagName` "WorldState.Health")) _result_2)))))

(fn `GetClosestEnemy`
  (params (ForAgent :type "BHGOAPAgent Interface (by ref)"))
  (returns (Found :type Boolean) (Enemy :type "Actor Object Reference") (Distance :type "Float (double-precision)"))
  (locals (LClosestDistance :type "Float (double-precision)") (LInstigatorActor :type "Actor Object Reference") (LClosestEnemy :type "/Game/Blueprints/BP_BHCharacterBase Object Reference"))
  (bind _output_get (set `local.LInstigatorActor` (cast `Actor` ForAgent :!pure true)))
  (bind _returnvalue (message `BHGOAPAgent.GetGOAPMemoryComponent` _output_get))
  (set `local.LClosestDistance` 99999999.0)
  (for _array_element (`BHMemoryComponent.GetMemory` _returnvalue)
    (bind _asbp_bhplayable_character (cast `/Game/Blueprints/BP_BHPlayableCharacter` _array_element))
    (bind (_bsuccessfullyfoundattribute _returnvalue_2) (`AbilitySystemBlueprintLibrary.GetFloatAttribute` _asbp_bhplayable_character (struct :`AttributeName` "Health" :`Attribute` "/Script/BrainHacker.BHAttributeSetBase:Health")))
    (if (and _bsuccessfullyfoundattribute (> _returnvalue_2 0.0))
      (bind _returnvalue_3 (`KismetMathLibrary.Vector_Distance` (`Actor.K2_GetActorLocation` _asbp_bhplayable_character) (`Actor.K2_GetActorLocation` (`local.LInstigatorActor`))))
      (if (< _returnvalue_3 (`local.LClosestDistance`))
        (set `local.LClosestDistance` _returnvalue_3)
        (set `local.LClosestEnemy` _asbp_bhplayable_character))))
  (return (`KismetSystemLibrary.IsValid` (`local.LClosestEnemy`)) (`local.LClosestEnemy`) (`local.LClosestDistance`)))

(fn `GetFearFactor`
  (returns (Result :type "Float (double-precision)"))
  (return (/ (`.ReturnValue` (`AbilitySystemBlueprintLibrary.GetFloatAttributeFromAbilitySystemComponent` (`AbilitySystemBlueprintLibrary.GetAbilitySystemComponent` (cast `Actor` (`self.AgentActor`) :!pure true)) (struct :`AttributeName` "Fear" :`Attribute` "/Script/BrainHacker.BHAttributeSetBase:Fear"))) 100.0)))

(fn `GetGoalScore`
  (returns (ReturnValue :type "Float (single-precision)"))
  (bind _found (`self.GetClosestEnemy` (`self.AgentActor`)))
  (if _found
    (if (or (> (`self.GetHealthFactor`) 0.5) (> (`self.GetFearFactor`) 0.5))
      (return 1.0)
      (else
        (return 0.0)))
    (else
      (return 0.0))))

(fn `GetHealthFactor`
  (returns (Result :type "Float (double-precision)"))
  (return (- 1.0 (/ (`.ReturnValue` (`AbilitySystemBlueprintLibrary.GetFloatAttributeFromAbilitySystemComponent` (`AbilitySystemBlueprintLibrary.GetAbilitySystemComponent` (cast `Actor` (`self.AgentActor`) :!pure true)) (struct :`AttributeName` "Health" :`Attribute` "/Script/BrainHacker.BHAttributeSetBase:Health"))) 100.0))))

(fn `IsGoalValid`
  (returns (ReturnValue :type Boolean))
  (return true))