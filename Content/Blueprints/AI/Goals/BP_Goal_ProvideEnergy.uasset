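; GOAP goal that has an AI agent provide energy to an energy storage that is not at full productivity.
; It searches the agent's GOAP memory for the first such BP_EnergyStorage and is valid only when one is found.
; The desired world state sets that storage's EnergyLevel key to DesiredEnergyLevel, and priority comes directly from the GoalScore variable.
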(event `self.UpdateDesiredWorldState`
  (bind (_found _energystorage) (`self.GetFirstEnergyStorage` (`self.AgentActor`)))
  (bind _result (`BHWorldStateFunctionLibrary.SetWorldStateValue` (`.WorldStateValue` (break `BHWorldStateData` (`self.DesiredWorldState`))) (`self.DesiredEnergyLevel`)))
  (set `self.DesiredWorldState` (make `BHWorldStateData` (make `BHWorldStateKey` _energystorage (struct :`TagName` "WorldState.EnergyLevel")) _result)))

(fn `GetFirstEnergyStorage`
  (params (ForAgent :type "BHGOAPAgent Interface (by ref)"))
  (returns (Found :type Boolean) (EnergyStorage :type "Actor Object Reference"))
  (locals (LInstigatorActor :type "Actor Object Reference"))
  (bind _output_get (set `local.LInstigatorActor` (cast `Actor` ForAgent :!pure true)))
  (bind _returnvalue (message `BHGOAPAgent.GetGOAPMemoryComponent` _output_get))
  (for _array_element (`BHMemoryComponent.GetMemory` _returnvalue)
    (bind _asbp_energy_storage (cast `/Game/Blueprints/BP_EnergyStorage` _array_element))
    (bind _result (`/Game/Blueprints/BP_EnergyStorage.IsFullProductivity` _asbp_energy_storage))
    (if (not _result)
      (return true _asbp_energy_storage)))
  (return false null))

(fn `GetGoalScore`
  (returns (ReturnValue :type "Float (single-precision)"))
  (return (`self.GoalScore`)))

(fn `IsGoalValid`
  (returns (ReturnValue :type Boolean))
  (bind (_found _energystorage) (`self.GetFirstEnergyStorage` (`self.AgentActor`)))
  (if _found
    (return (`KismetSystemLibrary.IsValid` _energystorage))
    (else
      (return false))))