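; GOAP goal that drives an AI agent toward computer work.
; It searches the agent's GOAP memory for a BP_Computer and is valid only when one is found.
; The desired world state pairs that computer and the WorldState.Activity tag with the DesiredActivity value.
; Its priority comes straight from the GoalScore variable, with no dynamic scoring.
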(event `self.UpdateDesiredWorldState`
  (bind (_found _computer) (`self.GetFirstComputer` (`self.AgentActor`)))
  (bind _result (`BHWorldStateFunctionLibrary.SetWorldStateValue` (`.WorldStateValue` (break `BHWorldStateData` (`self.DesiredWorldState`))) (`self.DesiredActivity`)))
  (set `self.DesiredWorldState` (make `BHWorldStateData` (make `BHWorldStateKey` _computer (struct :`TagName` "WorldState.Activity")) _result)))

(fn `GetFirstComputer`
  (params (ForAgent :type "BHGOAPAgent Interface (by ref)"))
  (returns (Found :type Boolean) (Computer :type "Actor Object Reference"))
  (locals (LInstigatorActor :type "Actor Object Reference"))
  (bind _output_get (set `local.LInstigatorActor` (cast `Actor` ForAgent :!pure true)))
  (bind _returnvalue (message `BHGOAPAgent.GetGOAPMemoryComponent` _output_get))
  (for _array_element (`BHMemoryComponent.GetMemory` _returnvalue)
    (bind _asbp_computer (cast `/Game/Blueprints/BP_Computer` _array_element))
    (return true _asbp_computer))
  (return false null))

(fn `GetGoalScore`
  (returns (ReturnValue :type "Float (double-precision)"))
  (return (`self.GoalScore`)))

(fn `IsGoalValid`
  (returns (ReturnValue :type Boolean))
  (bind (_found _computer) (`self.GetFirstComputer` (`self.AgentActor`)))
  (if _found
    (return (`KismetSystemLibrary.IsValid` _computer))
    (else
      (return false))))