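; GOAP-style AI goal that makes an NPC investigate when another character it remembers is alerted.
; It is valid only while the agent's own IsAlerted world state is false and some NPC in its BHMemory reports IsAlerted as true.
; The desired world state sets the agent's IsAlerted key to a configurable value, and the score is the GoalScore variable.
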(event `self.UpdateDesiredWorldState`
  (bind _result (`BHWorldStateFunctionLibrary.SetWorldStateValue` (`.WorldStateValue` (break `BHWorldStateData` (`self.DesiredWorldState`))) (`self.DesiredIsAlertedState`)))
  (set `self.DesiredWorldState` (make `BHWorldStateData` (make `BHWorldStateKey` (cast `Actor` (`self.AgentActor`) :!pure true) (struct :`TagName` "WorldState.IsAlerted")) _result)))

(fn `GetGoalScore`
  (returns (ReturnValue :type "Float (single-precision)"))
  (return (`self.GoalScore`)))

(fn `IsGoalValid`
  (returns (ReturnValue :type Boolean))
  (bind _asbp_bhnpccharacter_base (cast `/Game/Blueprints/BP_BHNPCCharacterBase` (`self.AgentActor`) :!pure true))
  (bind _returnvalue (`BHWorldStateProvider.GetWorldStateValue` (`BrainHackerCharacter.WorldStateProvider` _asbp_bhnpccharacter_base) (struct :`TagName` "WorldState.IsAlerted")))
  (bind _returnvalue_2 (`BHWorldStateFunctionLibrary.GetWorldStateValueAsBool` _returnvalue))
  (if (not _returnvalue_2)
    (for _array_element (`BHMemoryComponent.GetMemory` (`/Game/Blueprints/BP_BHNPCCharacterBase.BHMemory` _asbp_bhnpccharacter_base))
      (bind _asbp_bhnpccharacter_base_2 (cast `/Game/Blueprints/BP_BHNPCCharacterBase` _array_element))
      (bind _worldstateprovider (`BrainHackerCharacter.WorldStateProvider` _asbp_bhnpccharacter_base_2))
      (bind _returnvalue_3 (`BHWorldStateProvider.HasWorldStateValue` _worldstateprovider (struct :`TagName` "WorldState.IsAlerted")))
      (if _returnvalue_3
        (bind _returnvalue_4 (`BHWorldStateProvider.GetWorldStateValue` _worldstateprovider (struct :`TagName` "WorldState.IsAlerted")))
        (bind _returnvalue_5 (`BHWorldStateFunctionLibrary.GetWorldStateValueAsBool` _returnvalue_4))
        (if _returnvalue_5
          (return true))))
    (return false)
    (else
      (return false))))