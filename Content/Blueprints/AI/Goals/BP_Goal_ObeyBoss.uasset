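; GOAP goal that makes an AI agent obey a boss NPC present in its memory.
; GetBossCharacter searches the agent's GOAP memory for a BP_BHNPC_Boss, which makes the goal valid and yields GoalScore, otherwise zero.
; The desired world state sets the boss's WaitForActor state to a null actor value.
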(event `self.UpdateDesiredWorldState`
  (bind (_found _boss) (`self.GetBossCharacter` (`self.AgentActor`)))
  (bind _result (`BHWorldStateFunctionLibrary.SetWorldStateValue` (`.WorldStateValue` (break `BHWorldStateData` (`self.DesiredWorldState`))) (`self.NullActor`)))
  (set `self.DesiredWorldState` (make `BHWorldStateData` (make `BHWorldStateKey` _boss (struct :`TagName` "WorldState.WaitForActor")) _result)))

(fn `GetBossCharacter`
  (params (ForAgent :type "BHGOAPAgent Interface (by ref)"))
  (returns (Found :type Boolean) (Boss :type "Actor Object Reference"))
  (locals (LInstigatorActor :type "Actor Object Reference"))
  (bind _output_get (set `local.LInstigatorActor` (cast `Actor` ForAgent :!pure true)))
  (bind _returnvalue (message `BHGOAPAgent.GetGOAPMemoryComponent` _output_get))
  (for _array_element (`BHMemoryComponent.GetMemory` _returnvalue)
    (bind _asbp_bhnpc_boss (cast `/Game/Blueprints/BP_BHNPC_Boss` _array_element))
    (return true _asbp_bhnpc_boss))
  (return false null))

(fn `GetGoalScore`
  (returns (ReturnValue :type "Float (single-precision)"))
  (bind _found (`self.GetBossCharacter` (`self.AgentActor`)))
  (if _found
    (return (`self.GoalScore`))
    (else
      (return 0.0))))

(fn `IsGoalValid`
  (returns (ReturnValue :type Boolean))
  (bind _found (`self.GetBossCharacter` (`self.AgentActor`)))
  (return _found))