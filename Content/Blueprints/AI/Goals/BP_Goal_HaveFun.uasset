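; BP_Goal_HaveFun is an AI planning goal that makes an agent want to have fun.
; It builds its desired world state from the WorldState.HasFun tag on the agent's actor, with the value taken from DesiredHasFunState.
; The goal is always valid and reports its GoalScore variable as priority without computing it from context.
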(event `self.UpdateDesiredWorldState`
  (bind _result (`BHWorldStateFunctionLibrary.SetWorldStateValue` (`.WorldStateValue` (break `BHWorldStateData` (`self.DesiredWorldState`))) (`self.DesiredHasFunState`)))
  (set `self.DesiredWorldState` (make `BHWorldStateData` (make `BHWorldStateKey` (cast `Actor` (`self.AgentActor`) :!pure true) (struct :`TagName` "WorldState.HasFun")) _result)))

(fn `GetGoalScore`
  (returns (ReturnValue :type "Float (double-precision)"))
  (return (`self.GoalScore`)))

(fn `IsGoalValid`
  (returns (ReturnValue :type Boolean))
  (return true))