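; World state atom that reports whether an AI NPC is alerted, meaning its memory holds a playable character.
; On each atom data update it resets the alerted flag, then scans the owning NPC's BHMemory entries.
; Any entry that casts to BP_BHPlayableCharacter sets the flag, and the result is written to the atom's world state value.
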(event `self.UpdateWorldStateAtomData`
  (set `self.bAlertedState` false)
  (for _array_element (`BHMemoryComponent.GetMemory` (`/Game/Blueprints/BP_BHNPCCharacterBase.BHMemory` (cast `/Game/Blueprints/BP_BHNPCCharacterBase` (`self.OwnerActor`) :!pure true)))
    (cast `/Game/Blueprints/BP_BHPlayableCharacter` _array_element)
    (set `self.bAlertedState` true))
  (`BHWorldStateFunctionLibrary.SetWorldStateValue` (`self.WorldStateValue`) (`self.bAlertedState`)))