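; BP_WSA_Location is an AI world state atom that records the location of its owner actor.
; On each data update it checks whether the owner implements BPI_ActivityObject.
; Activity objects supply their interaction location through an interface message, while any other owner uses its actor location.
; The chosen location is written into the atom's world state value.
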(event `self.UpdateWorldStateAtomData`
  (if (`KismetSystemLibrary.DoesImplementInterface` (`self.OwnerActor`) "/Game/Blueprints/BPI_ActivityObject.BPI_ActivityObject_C")
    (bind _result (message `/Game/Blueprints/BPI_ActivityObject.GetInteractionLocation` (`self.OwnerActor`)))
    (`BHWorldStateFunctionLibrary.SetWorldStateValue` (`self.WorldStateValue`) _result)
    (else
      (`BHWorldStateFunctionLibrary.SetWorldStateValue` (`self.WorldStateValue`) (`Actor.K2_GetActorLocation` (`self.OwnerActor`))))))