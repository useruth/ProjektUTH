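; Base NPC character Blueprint that wires up GOAP memory and planner components, an enemy panel widget and emissive color control.
; BeginPlay temporarily seeds BHMemory with every other NPC, battery, generator, computer and energy storage, then initializes the panel after a short delay.
; It also replaces mesh materials with dynamic instances and caches their emissive colors, so SetEmissiveColor can tint them and ResetEmissiveColor can restore defaults.
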(event `self.ReceiveBeginPlay`
  (`parent.ReceiveBeginPlay`)
  (`|ExecutionSequence`
    (:`then_0`
      ;[1 1 1] add initial memory (temporary)
      (`|ExecutionSequence`
        (:`then_0`
          (bind _outactors (`GameplayStatics.GetAllActorsOfClass` "BP_BHNPCCharacterBase_C"))
          (for _array_element _outactors
            (if (!= _array_element self)
              (`BHMemoryComponent.RegisterActorInMemory` (`self.BHMemory`) _array_element))))
        (:`then_1`
          (bind _outactors_2 (`GameplayStatics.GetAllActorsOfClass` "/Game/Blueprints/BP_Battery.BP_Battery_C"))
          (for _array_element_2 _outactors_2
            (`BHMemoryComponent.RegisterActorInMemory` (`self.BHMemory`) _array_element_2)))
        (:`then_2`
          (bind _outactors_3 (`GameplayStatics.GetAllActorsOfClass` "/Game/Blueprints/BP_Generator.BP_Generator_C"))
          (for _array_element_3 _outactors_3
            (`BHMemoryComponent.RegisterActorInMemory` (`self.BHMemory`) _array_element_3)))
        (:`then_3`
          (bind _outactors_4 (`GameplayStatics.GetAllActorsOfClass` "/Game/Blueprints/BP_Computer.BP_Computer_C"))
          (for _array_element_4 _outactors_4
            (`BHMemoryComponent.RegisterActorInMemory` (`self.BHMemory`) _array_element_4)))
        (:`then_4`
          (bind _outactors_5 (`GameplayStatics.GetAllActorsOfClass` "/Game/Blueprints/BP_EnergyStorage.BP_EnergyStorage_C"))
          (for _array_element_5 _outactors_5
            (`BHMemoryComponent.RegisterActorInMemory` (`self.BHMemory`) _array_element_5)))))
    (:`then_1`
      ;[1 1 1] initialize enemy panel widget
      (`KismetSystemLibrary.Delay` 0.2)
      (`/Game/Widgets/WBP_EnemyPanel.InitWithCharacter` (cast `/Game/Widgets/WBP_EnemyPanel` (`WidgetComponent.GetUserWidgetObject` (`self.EnemyPanel`)) :!pure true) self))
    (:`then_2`
      ;[1 1 1] create dynamic materials instances
      (for _array_element_6 (`MeshComponent.GetMaterials` (`self.Mesh`))
        (bind _returnvalue (`KismetMaterialLibrary.CreateDynamicMaterialInstance` _array_element_6))
        (bind _returnvalue_2 (`KismetArrayLibrary.Array_Add` (`self.DynamicMaterialsInstances`) _returnvalue))
        (`PrimitiveComponent.SetMaterial` (`self.Mesh`) _returnvalue_2 _returnvalue)))
    (:`then_3`
      ;[1 1 1] cache defaults emissive colors
      (for _array_element_7 (`self.DynamicMaterialsInstances`)
        (bind _returnvalue_3 (`MaterialInstanceDynamic.K2_GetVectorParameterValue` _array_element_7 "EmissiveColor"))
        (`KismetArrayLibrary.Array_Add` (`self.DefaultsEmissiveColors`) _returnvalue_3)))))

(fn `GetGOAPMemoryComponent`
  (returns (ReturnValue :type "BHMemoryComponent Object Reference"))
  (return (`self.BHMemory`)))

(fn `GetGOAPPlanner`
  (returns (ReturnValue :type "BHPlanner Object Reference"))
  (return (`self.BHPlanner`)))

(fn `ResetEmissiveColor`
  (for (_array_element _array_index) (`self.DynamicMaterialsInstances`)
    (`MaterialInstanceDynamic.SetVectorParameterValue` _array_element "EmissiveColor" (`|GetArrayItem` (`self.DefaultsEmissiveColors`) _array_index))))

(fn `SetEmissiveColor`
  (params (Color :type "LinearColor Structure"))
  (for _array_element (`self.DynamicMaterialsInstances`)
    (`MaterialInstanceDynamic.SetVectorParameterValue` _array_element "EmissiveColor" Color)))

(fn `UserConstructionScript`
  (`parent.UserConstructionScript`))