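; BP_EnergyStorage is an energy storage Blueprint that holds a CurrentEnergy pool and tracks a set of linked power generators.
; AddEnergy and ConsumeEnergy act only on crossings of zero, firing a state-changed event dispatcher and swapping the mesh's active/inactive material.
; Running empty also deactivates every linked generator, while refilling does not reactivate them.
; IsFullProductivity reports whether all linked generators are active.
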(event `self.ReceiveTick`
  (params (DeltaSeconds :type "Float (single-precision)")))

(fn `AddEnergy`
  (params (Energy :type "Float (double-precision)"))
  (locals (LOldState :type "Float (double-precision)" :default 0.0))
  (set `local.LOldState` (`self.CurrentEnergy`))
  (set `self.CurrentEnergy` (+ Energy (`self.CurrentEnergy`)))
  (if (and (<= (`local.LOldState`) 0.0) (> (`self.CurrentEnergy`) 0.0))
    (`|ExecutionSequence`
      (:`then_0`
        (`self.EnergyStorageStateChangedED` true))
      (:`then_1`
        (`PrimitiveComponent.SetMaterial` (`self.StaticMesh`) 0 (`self.ActiveMatarial`))))))

(fn `ConsumeEnergy`
  (params (Amount :type "Float (double-precision)"))
  (locals (LOldState :type "Float (double-precision)" :default 0.0))
  (set `local.LOldState` (`self.CurrentEnergy`))
  (set `self.CurrentEnergy` (`KismetMathLibrary.FMax` (- (`self.CurrentEnergy`) Amount)))
  (if (and (> (`local.LOldState`) 0.0) (<= (`self.CurrentEnergy`) 0.0))
    (`|ExecutionSequence`
      (:`then_0`
        (for _array_element (`self.PowerGenerators`)
          (`/Game/Blueprints/BP_Generator.SetIsActive` _array_element false))
        (`self.EnergyStorageStateChangedED` false))
      (:`then_1`
        (`PrimitiveComponent.SetMaterial` (`self.StaticMesh`) 0 (`self.InactiveMatarial`))))))

(fn `IsFullProductivity`
  (returns (Result :type Boolean))
  (for _array_element (`self.PowerGenerators`)
    (bind _result (`/Game/Blueprints/BP_Generator.GetIsActive` _array_element))
    (if (not _result)
      (return false)))
  (return true))

(fn `UserConstructionScript`)