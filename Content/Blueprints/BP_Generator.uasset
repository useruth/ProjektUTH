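; BP_Generator is a switchable generator actor that adds an energy boost to its EnergyStorage each time it is set active.
; Setting the state also swaps the mesh material between active and inactive and prints an ENABLED/DISABLED message.
; It exposes getters for active state and interaction location, names the first BP_Battery found in the level as its required object, and stores a HasBattery flag that activation does not check.
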(event `/Game/Blueprints/BPI_ActivityObject.SetIsActive`
  (params (Active :type Boolean))
  (`|ExecutionSequence`
    (:`then_0`
      (bind _output_get (set `self.IsGeneratorEnabled` Active))
      (if _output_get
        (`/Game/Blueprints/BP_EnergyStorage.AddEnergy` (`self.EnergyStorage`) (`self.EnergyBoost`))))
    (:`then_1`
      (`PrimitiveComponent.SetMaterial` (`self.StaticMesh`) 0 (select `bool` (`self.IsGeneratorEnabled`) :`false` (`self.InactiveMatarial`) :`true` (`self.ActiveMatarial`) :!type "MaterialInterface Object Reference")))
    (:`then_2`
      (`KismetSystemLibrary.PrintString` (`KismetMathLibrary.SelectString` "ENABLED" "DISABLED" (`self.IsGeneratorEnabled`)) true true (struct :`R` 1.0 :`A` 1.0) 6.0))))

(fn `GetGeneratorHasBattery`
  (returns (Result :type Boolean))
  (return (`self.HasBattery`)))

(fn `GetInteractionLocation`
  (returns (Result :type "Vector Structure"))
  (return (`SceneComponent.K2_GetComponentLocation` (`self.InteractionLocation`))))

(fn `GetIsActive`
  (returns (Result :type Boolean))
  (return (`self.IsGeneratorEnabled`)))

(fn `GetRequiredObject`
  (returns (Result :type "/Game/Blueprints/BP_Battery Object Reference"))
  (bind _outactors (`GameplayStatics.GetAllActorsOfClass` "/Game/Blueprints/BP_Battery.BP_Battery_C"))
  (return (`|GetArrayItem` _outactors)))

(fn `SetGeneratorHasBattery`
  (params (HasBattery :type Boolean))
  (set `self.HasBattery` HasBattery))

(fn `UserConstructionScript`)